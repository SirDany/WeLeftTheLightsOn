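; Player state that holds the player's stats and active effects, including those behind hunger and thirst.
; Stats start from a data table, and each tick external helpers update effects, then stats, then evaluate hunger and thirst.
; Update functions merge incoming arrays by type through maps, drop effects without stacks, and broadcast the results.
; Getters return type-filtered maps, and ResetPlayer resets and reinitializes stats.
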(event `self.ReceiveBeginPlay`
  (`self.InitializePlayerStats`))

(event `self.ReceiveTick`
  (params (DeltaSeconds :type "Float (single-precision)"))
  (`/Game/Players/EffectsSystem/BPFL_EffectService.UpdateActiveEffectsOnTick` DeltaSeconds self)
  (`/Game/Players/StatSystem/BPFL_PlayerStatService.UpdatePlayerStatsOnTick` DeltaSeconds self)
  (`/Game/Players/StatSystem/BPFL_PlayerStatService.EvaluateHungerAndThirst` self))

(fn `GetActiveEffectsByType`
  (params (Types :type "Array of /Game/Players/EffectsSystem/Data/EN_EffectType Enum"))
  (returns (ActiveEffects :type "Map of /Game/Players/EffectsSystem/Data/EN_EffectType Enum to /Game/Players/EffectsSystem/Data/ST_ActiveEffect Structure"))
  (locals (ActiveEffectsMap :type "Map of /Game/Players/EffectsSystem/Data/EN_EffectType Enum to /Game/Players/EffectsSystem/Data/ST_ActiveEffect Structure"))
  (for _array_element (`self.ActiveEffects`)
    (bind _effecttype (break `/Game/Players/EffectsSystem/Data/ST_ActiveEffect` _array_element))
    (if (or (`KismetArrayLibrary.Array_IsEmpty` Types) (`KismetArrayLibrary.Array_Contains` Types _effecttype))
      (`BlueprintMapLibrary.Map_Add` (`local.ActiveEffectsMap`) _effecttype _array_element)))
  (return (`local.ActiveEffectsMap`)))

(fn `GetEffectsData`
  (returns (EffectsDataTable :type "DataTable Object Reference"))
  (return (`self.EffectsDataTable`)))

(fn `GetPlayerStatsByType`
  (params (Types :type "Array of /Game/Players/StatSystem/EN_PlayerStatType Enum"))
  (returns (PlayerStats :type "Map of /Game/Players/StatSystem/EN_PlayerStatType Enum to /Game/Players/StatSystem/ST_PlayerStat Structure"))
  (locals (PlayerStatsMap :type "Map of /Game/Players/StatSystem/EN_PlayerStatType Enum to /Game/Players/StatSystem/ST_PlayerStat Structure"))
  (for _array_element (`self.Stats`)
    (bind (_current _max _rate _type) (break `/Game/Players/StatSystem/ST_PlayerStat` _array_element))
    (if (or (`KismetArrayLibrary.Array_IsEmpty` Types) (`KismetArrayLibrary.Array_Contains` Types _type))
      (`BlueprintMapLibrary.Map_Add` (`local.PlayerStatsMap`) _type _array_element)))
  (return (`local.PlayerStatsMap`)))

(fn `InitializePlayerStats`
  (bind _playerstatsdatatable (`self.PlayerStatsDataTable`))
  (bind _outrownames (`DataTableFunctionLibrary.GetDataTableRowNames` _playerstatsdatatable))
  (for _array_element _outrownames
    (bind _returnvalue (`|GetDataTableRow` _playerstatsdatatable _array_element)
      (:`then`
        (bind (_basemax _baserate _playerstattype) (break `/Game/Players/StatSystem/ST_PlayerStatsRow` _returnvalue))
        (`KismetArrayLibrary.Array_Add` (`self.Stats`) (make `/Game/Players/StatSystem/ST_PlayerStat` _basemax _basemax _baserate _playerstattype))))))

(fn `ResetPlayer`
  (`/Game/Players/StatSystem/BPFL_PlayerStatService.ResetAllStats` self)
  (`self.InitializePlayerStats`))

(fn `ResetPlayerEffects`
  (`KismetArrayLibrary.Array_Clear` (`self.ActiveEffects`)))

(fn `ResetPlayerStats`
  (`KismetArrayLibrary.Array_Clear` (`self.Stats`)))

(fn `UpdateActiveEffects`
  (params (NewActiveEffects :type "Array of /Game/Players/EffectsSystem/Data/ST_ActiveEffect Structure"))
  (locals (ActiveEffectsMap :type "Map of /Game/Players/EffectsSystem/Data/EN_EffectType Enum to /Game/Players/EffectsSystem/Data/ST_ActiveEffect Structure"))
  (bind _activeeffects (`self.ActiveEffects`))
  (bind _activeeffectsmap (`local.ActiveEffectsMap`))
  ; Prevent empty updates
  (if (or (> (`KismetArrayLibrary.Array_Length` _activeeffects) 0) (> (`KismetArrayLibrary.Array_Length` NewActiveEffects) 0))
    ; Create map of current effects for simple lookup
    (for _array_element _activeeffects
      (`BlueprintMapLibrary.Map_Add` _activeeffectsmap (`.EffectType_8_815619CB407BC48AC54DD5AEF5E13A84` (break `/Game/Players/EffectsSystem/Data/ST_ActiveEffect` _array_element)) _array_element))
    (for _array_element_2 NewActiveEffects
      (bind (_effecttype _currentstacks) (break `/Game/Players/EffectsSystem/Data/ST_ActiveEffect` _array_element_2))
      ; Filter out decayed effects
      (if (<= _currentstacks 0)
        (if (`.ReturnValue` (`BlueprintMapLibrary.Map_Find` _activeeffectsmap _effecttype))
          (`BlueprintMapLibrary.Map_Remove` _activeeffectsmap _effecttype))
        (else
          ; Add or update effects
          (`BlueprintMapLibrary.Map_Add` _activeeffectsmap _effecttype _array_element_2))))
    ; Set & send update event
    (bind _values (`BlueprintMapLibrary.Map_Values` _activeeffectsmap))
    (bind _output_get (set `self.ActiveEffects` _values))
    (`self.OnActiveEffectsUpdated` _output_get)))

(fn `UpdatePlayerStats`
  (params (NewPlayerStats :type "Array of /Game/Players/StatSystem/ST_PlayerStat Structure"))
  (locals (PlayerStatMap :type "Map of /Game/Players/StatSystem/EN_PlayerStatType Enum to /Game/Players/StatSystem/ST_PlayerStat Structure"))
  (bind _stats (`self.Stats`))
  (bind _playerstatmap (`local.PlayerStatMap`))
  ; Prevent empty updates
  (if (or (> (`KismetArrayLibrary.Array_Length` _stats) 0) (> (`KismetArrayLibrary.Array_Length` NewPlayerStats) 0))
    ; Create map of current stats for simple lookup
    (for _array_element _stats
      (`BlueprintMapLibrary.Map_Add` _playerstatmap (`.Type_12_9D0B473A4B87CB9531C890AB77D992B4` (break `/Game/Players/StatSystem/ST_PlayerStat` _array_element)) _array_element))
    ; Update or add stats
    (for _array_element_2 NewPlayerStats
      (`BlueprintMapLibrary.Map_Add` _playerstatmap (`.Type_12_9D0B473A4B87CB9531C890AB77D992B4` (break `/Game/Players/StatSystem/ST_PlayerStat` _array_element_2)) _array_element_2))
    (bind _values (`BlueprintMapLibrary.Map_Values` _playerstatmap))
    (bind _output_get (set `self.Stats` _values))
    (`self.OnPlayerStatsUpdated` _output_get) ; Ignore the pass by reference note, arrays will still be passed even as non reference.
  ))

(fn `UserConstructionScript`)