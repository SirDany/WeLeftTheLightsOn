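; Job manager component that handles offering, accepting, tracking, completing and abandoning the player's single active job.
; Each operation reads job or ship state structs and writes modified copies back through update functions.
; Accepting a job spends ship energy; completion requires all mandatory objectives and pays money for completed ones.
; Item progress goes to the first unfinished matching objective, mandatory before optional, clamped at its required amount.
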(fn `AbandonActiveJob`
  (returns (Success :type Boolean))
  (bind (_jobstate _success) (`self.GetJobState`))
  (if _success
    (if (`.HasActiveJob_13_0208072C43EEBF76856A8C91F30FADC0` (break `/Game/Systems/Jobs/ST_JobState` _jobstate))
      (bind _structout (setmembers `/Game/Systems/Jobs/ST_JobState` :`StructRef` _jobstate :`HasActiveJob` false))
      (bind _success_2 (`self.UpdateJobState` _structout))
      (return _success_2)
      (else
        _)))
  (return false))

(fn `CompleteActiveJob`
  (returns (Success :type Boolean))
  (locals (Rewards :type "Array of /Game/Systems/Jobs/JobStructs/ST_Reward Structure"))
  (bind (_jobstate _success) (`self.GetJobState`))
  (if _success
    (bind ((`ActiveJob_2_5472E60E4AB6179533702CB83EDF4A6F` _activejob) (`HasActiveJob_13_0208072C43EEBF76856A8C91F30FADC0` _hasactivejob)) (break `/Game/Systems/Jobs/ST_JobState` _jobstate))
    (if _hasactivejob
      ; Check objective status & gat rewards
      (for _array_element (`.Objectives_16_67BC31FC48D4DEAE86676DB1571AA7AA` (break `/Game/Systems/Jobs/JobStructs/ST_Job` _activejob))
        (bind ((`Reward_31_B6C3DC8241464738BE2C2C9E432D2434` _reward) (`IsOptional_26_8ABF692140C9E4325F11D994841A4F82` _isoptional) (`CompletionDetails_30_B6FC68DA4DB95CDD6BC0709F3FD1A4B5` _completiondetails)) (break `/Game/Systems/Jobs/JobStructs/ST_Objective` _array_element))
        (bind ((`IsCompleted_1_894D2C4D4EFA0CC57DBB40887E524427` _iscompleted)) (break `/Game/Systems/Jobs/JobStructs/ST_CompletionDetails` _completiondetails))
        (if (and (not _isoptional) (not _iscompleted))
          (`/Game/Utils/BPFL_Logging.Warn` self "All mandatory objectives must be completed first!" "CompleteActiveJob")
          (return false)
          (elif _iscompleted
            (`KismetArrayLibrary.Array_Add` (`local.Rewards`) _reward))))
      ; Complete job & update job state
      (bind _structout (setmembers `/Game/Systems/Jobs/ST_JobState` :`StructRef` _jobstate :`HasActiveJob` false))
      (bind _success_2 (`self.UpdateJobState` _structout))
      (if _success_2
        (bind _success_3 (`self.DistributeRewards` (`local.Rewards`)))
        (return _success_3)
        (else
          (return false)))
      (else
        _)))
  (return false))

(fn `DistributeRewards`
  (params (Rewards :type "Array of /Game/Systems/Jobs/JobStructs/ST_Reward Structure"))
  (returns (Success :type Boolean))
  (locals (TotalMoneyReward :type Integer))
  (bind _totalmoneyreward (`local.TotalMoneyReward`))
  (bind (_shipstate _success) (`self.GetShipState`))
  (if _success
    ; Calculate reward money
    (for _array_element Rewards
      (set `local.TotalMoneyReward` (+ (`.Money_2_AFA861594D57F02B5B5D77BABEF9E904` (break `/Game/Systems/Jobs/JobStructs/ST_Reward` _array_element)) _totalmoneyreward)))
    ; Update Ship State
    (bind _structout (setmembers `/Game/Systems/Ship/ST_ShipState` :`StructRef` _shipstate :`Money` (+ _totalmoneyreward (`.Money_5_7DF295D4402D080029653BA6F690F0BE` (break `/Game/Systems/Ship/ST_ShipState` _shipstate)))))
    (bind _success_2 (`self.UpdateShipState` _structout))
    (if _success_2
      (return true)
      (else
        _)))
  (`/Game/Utils/BPFL_Logging.Warn` self "Failed to distribute rewards!" "CompleteActiveJob")
  (return false))

(fn `GetAvailableJobs`
  (returns (AvailableJobs :type "Array of /Game/Systems/Jobs/JobStructs/ST_Job Structure") (HasAvailableJobs :type Boolean))
  (bind _jobstate (`self.GetJobState`))
  (bind (_activejob _availablejobs _hasactivejob _hasavailablejobs) (break `/Game/Systems/Jobs/ST_JobState` _jobstate))
  (return _availablejobs _hasavailablejobs))

(fn `GetJob`
  (params (ID :type Name))
  (returns (Job :type "/Game/Systems/Jobs/JobStructs/ST_Job Structure") (`Job Found` :type Boolean))
  (bind (_jobstate _success) (`self.GetJobState`))
  (if _success
    (bind (_activejob _availablejobs _hasactivejob _hasavailablejobs) (break `/Game/Systems/Jobs/ST_JobState` _jobstate))
    ; Active job match
    (if (and (== (`.ID_27_6A91DE8C46E46007FA636AAEA33E7B4E` (break `/Game/Systems/Jobs/JobStructs/ST_Job` _activejob)) (`local.ID`)) _hasactivejob)
      (return _activejob true)
      (elif _hasavailablejobs
        ; Find in available jobs
        (for _array_element _availablejobs
          (if (== (`.ID_27_6A91DE8C46E46007FA636AAEA33E7B4E` (break `/Game/Systems/Jobs/JobStructs/ST_Job` _array_element)) (`local.ID`))
            (return _array_element true))))))
  ; No job found
  (`/Game/Utils/BPFL_Logging.Warn` self (`|FormatText` "Could not find job: {jobid}" (`local.ID`)) "GetJob")
  (return (struct) false))

(fn `GetRemainingObjectiveItems`
  (returns (Items :type "Map of Name to Integer"))
  (locals (ItemAmountsMap :type "Map of Name to Object Object Reference"))
  (bind (_jobstate _success) (`self.GetJobState`))
  (bind ((`ActiveJob_2_5472E60E4AB6179533702CB83EDF4A6F` _activejob) (`HasActiveJob_13_0208072C43EEBF76856A8C91F30FADC0` _hasactivejob)) (break `/Game/Systems/Jobs/ST_JobState` _jobstate))
  (if (and _hasactivejob _success)
    (for _array_element (`.Objectives_16_67BC31FC48D4DEAE86676DB1571AA7AA` (break `/Game/Systems/Jobs/JobStructs/ST_Job` _activejob))
      (bind (_iscompleted _pickupitemid _requiredamount _currentamount) (break `/Game/Systems/Jobs/JobStructs/ST_CompletionDetails` (`.CompletionDetails_30_B6FC68DA4DB95CDD6BC0709F3FD1A4B5` (break `/Game/Systems/Jobs/JobStructs/ST_Objective` _array_element))))
      (if (not _iscompleted)
        (`BlueprintMapLibrary.Map_Add` (`local.ItemAmountsMap`) _pickupitemid (- _requiredamount _currentamount))))
    (return (`local.ItemAmountsMap`))))

(fn `SetActiveJob`
  (params (ID :type Name))
  (returns (Success :type Boolean))
  ; Get required states
  (bind (_jobstate _success) (`self.GetJobState`))
  (bind (_shipstate _success_2) (`self.GetShipState`))
  (if (or (not _success_2) (not _success))
    _
    (elif (`.HasActiveJob_13_0208072C43EEBF76856A8C91F30FADC0` (break `/Game/Systems/Jobs/ST_JobState` _jobstate))
      (`/Game/Utils/BPFL_Logging.Info` self "Selected Job cannot override active job. Active Job must be abandoned first." "SetActiveJob")
      (else
        (bind (_job _job_found) (`self.GetJob` (`local.ID`)))
        (if _job_found
          (bind ((`Energy_2_AA8D4D8E454FA23F5F625AB9B92FAC67` _energy)) (break `/Game/Systems/Ship/ST_ShipState` _shipstate))
          (bind ((`EnergyCost_18_96FB950542B8FE18B58A3E9A4408EC9E` _energycost)) (break `/Game/Systems/Jobs/JobStructs/ST_Job` _job))
          ; Check & adjust ship energy
          (if (< _energy _energycost)
            (`/Game/Utils/BPFL_Logging.Info` self "Insufficient energy!" "SetActiveJob")
            (return false)
            (else
              (bind _structout (setmembers `/Game/Systems/Ship/ST_ShipState` :`StructRef` _shipstate :`Energy` (- _energy _energycost)))
              (`self.UpdateShipState` _structout)
              ; Update Job State
              (bind _structout_2 (setmembers `/Game/Systems/Jobs/ST_JobState` :`StructRef` _jobstate :`ActiveJob` _job :`AvailableJobs` (`|MakeArray` (struct) :!type "/Game/Systems/Jobs/JobStructs/ST_Job Structure") :`HasActiveJob` true :`HasAvailableJobs` false))
              (bind _success_3 (`self.UpdateJobState` _structout_2))
              (return _success_3)))
          (else
            _)))))
  (return false))

(fn `SetAvailableJobs`
  (params (NewJobs :type "Array of /Game/Systems/Jobs/JobStructs/ST_Job Structure"))
  (returns (Success :type Boolean))
  (bind (_jobstate _success) (`self.GetJobState`))
  (if _success
    (bind _structout (setmembers `/Game/Systems/Jobs/ST_JobState` :`StructRef` _jobstate :`AvailableJobs` NewJobs :`HasAvailableJobs` true))
    (bind _success_2 (`self.UpdateJobState` _structout))
    (return _success_2)
    (else
      (`/Game/Utils/BPFL_Logging.Error` null "Failed to set available jobs!" "SetAvailableJobs")
      (return false))))

(fn `TryGetFirstObjectiveByItemID`
  (params (ST_Job :type "/Game/Systems/Jobs/JobStructs/ST_Job Structure (by ref)") (ItemID :type Name))
  (returns (Objective :type "/Game/Systems/Jobs/JobStructs/ST_Objective Structure") (Index :type Integer) (ObjectiveFound :type Boolean))
  (locals (IsFirstMandatoryObjectiveFound :type Boolean) (IsFirstOptionalObjectiveFound :type Boolean) (FirstMandatoryObjective :type "/Game/Systems/Jobs/JobStructs/ST_Objective Structure") (FirstOptionalObjective :type "/Game/Systems/Jobs/JobStructs/ST_Objective Structure") (MandatoryIndex :type Integer) (OptionalIndex :type Integer))
  (for (_array_element _array_index) (`.Objectives_16_67BC31FC48D4DEAE86676DB1571AA7AA` (break `/Game/Systems/Jobs/JobStructs/ST_Job` ST_Job))
    (bind (_title _description _type _reward _isoptional _completiondetails) (break `/Game/Systems/Jobs/JobStructs/ST_Objective` _array_element))
    (bind (_iscompleted _pickupitemid) (break `/Game/Systems/Jobs/JobStructs/ST_CompletionDetails` _completiondetails))
    (bind _returnvalue (and (not _iscompleted) (== _pickupitemid (`local.ItemID`))))
    ; Check for first optional match
    (if (and (not (`local.IsFirstOptionalObjectiveFound`)) _isoptional _returnvalue)
      (set `local.FirstOptionalObjective` _array_element)
      (set `local.IsFirstOptionalObjectiveFound` true)
      (set `local.OptionalIndex` _array_index)
      (else
        ; Check for first mandatory match
        (if (and (not _isoptional) _returnvalue (not (`local.IsFirstMandatoryObjectiveFound`)))
          (set `local.FirstMandatoryObjective` _array_element)
          (set `local.IsFirstMandatoryObjectiveFound` true)
          (set `local.MandatoryIndex` _array_index)))))
  ; Return first mandatory match if found
  (if (`local.IsFirstMandatoryObjectiveFound`)
    (return (`local.FirstMandatoryObjective`) (`local.MandatoryIndex`) true)
    (else
      ; Return first optional match if found
      (if (`local.IsFirstOptionalObjectiveFound`)
        (return (`local.FirstOptionalObjective`) (`local.OptionalIndex`) true)
        (else
          (return (struct) 0 false))))))

(fn `UpdateJobProgress`
  (params (Amount :type Integer) (ItemID :type Name))
  (returns (Success :type Boolean))
  (locals (UpdatedJobObjectives :type "Array of /Game/Systems/Jobs/JobStructs/ST_Objective Structure"))
  (bind (_jobstate _success) (`self.GetJobState`))
  (bind ((`ActiveJob_2_5472E60E4AB6179533702CB83EDF4A6F` _activejob) (`HasActiveJob_13_0208072C43EEBF76856A8C91F30FADC0` _hasactivejob)) (break `/Game/Systems/Jobs/ST_JobState` _jobstate))
  (if (and _success _hasactivejob)
    ; Update progress in completion details of found objective
    (bind (_objective _index _objectivefound) (`self.TryGetFirstObjectiveByItemID` _activejob ItemID))
    (if _objectivefound
      (bind ((`CompletionDetails_30_B6FC68DA4DB95CDD6BC0709F3FD1A4B5` _completiondetails)) (break `/Game/Systems/Jobs/JobStructs/ST_Objective` _objective))
      (bind (_iscompleted _pickupitemid _requiredamount _currentamount) (break `/Game/Systems/Jobs/JobStructs/ST_CompletionDetails` _completiondetails))
      (bind _returnvalue (`KismetMathLibrary.Clamp` (+ _currentamount (`local.Amount`)) _currentamount _requiredamount))
      (bind _structout (setmembers `/Game/Systems/Jobs/JobStructs/ST_CompletionDetails` :`StructRef` _completiondetails :`IsCompleted` (== _requiredamount _returnvalue) :`CurrentAmount` _returnvalue))
      (bind _structout_2 (setmembers `/Game/Systems/Jobs/JobStructs/ST_Objective` :`StructRef` _objective :`CompletionDetails` _structout))
      ; Update job state
      (bind _output_get (set `local.UpdatedJobObjectives` (`.Objectives_16_67BC31FC48D4DEAE86676DB1571AA7AA` (break `/Game/Systems/Jobs/JobStructs/ST_Job` _activejob))))
      (`KismetArrayLibrary.Array_Set` _output_get _index _structout_2)
      (bind _structout_3 (setmembers `/Game/Systems/Jobs/JobStructs/ST_Job` :`StructRef` _activejob :`Objectives` _output_get))
      (bind _structout_4 (setmembers `/Game/Systems/Jobs/ST_JobState` :`StructRef` _jobstate :`ActiveJob` _structout_3))
      (bind _success_2 (`self.UpdateJobState` _structout_4))
      (if _success_2
        (return true)
        (else
          (`/Game/Utils/BPFL_Logging.Error` self "Failed to update Job Progress" "UpdateJobProgress")
          (return false))))
    (else
      (return false))))