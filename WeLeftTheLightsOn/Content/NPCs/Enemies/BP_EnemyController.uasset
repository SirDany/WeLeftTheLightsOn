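; AI controller for enemies that drives patrol and player chase through a behavior tree and blackboard.
; On BeginPlay it starts the base enemy tree and seeds the patrol target from the controlled character.
; Perception sets the target actor and HasTarget when the first-person player is sensed.
; Forgotten perception and failed moves share an update setting HasTarget false, which reads the forgotten event's actor and leaves the target key uncleared for players.
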(event `self.AIPerception.OnTargetPerceptionForgotten`
  (params (Actor :type "Actor Object Reference"))
  ; Reset chase when not possible or frogotten
  (`self.UpdateHasTarget` Actor :!label _label))

(event `ReceiveMoveCompleted_Event` :!signature `self.ReceiveMoveCompleted`
  (params (RequestID :type "AIRequestID Structure") (Result :type "EPathFollowingResult Enum" :default "Success"))
  ; Reset chase when not possible or frogotten
  (switch `EPathFollowingResult` Result
    (:`Blocked`
      (goto _label))
    (:`OffPath`
      (goto _label))
    (:`Aborted`
      (goto _label))
    (:`Invalid`
      (goto _label))))

(event `self.ReceiveBeginPlay`
  (`self.InitializeBehaviorTree`)
  (add `self.ReceiveMoveCompleted` (delegate `ReceiveMoveCompleted_Event`)))

(event `self.AIPerception.OnTargetPerceptionUpdated`
  (params (Actor :type "Actor Object Reference") (Stimulus :type "AIStimulus Structure"))
  (if (`.bSuccessfullySensed` (break `AIStimulus` Stimulus))
    (`self.UpdateHasTarget` Actor true)))

(fn `InitializeBehaviorTree`
  (bind (_blackboardcomponent _returnvalue) (`self.UseBlackboard` "/Game/NPCs/Enemies/Behavior/BB_EnemyBase.BB_EnemyBase"))
  (if _returnvalue
    (bind _returnvalue_2 (`self.RunBehaviorTree` "/Game/NPCs/Enemies/Behavior/BT_EnemyBase.BT_EnemyBase"))
    (if _returnvalue_2
      (bind _asbp_enemy_base_character (cast `/Game/NPCs/Enemies/BP_EnemyBaseCharacter` (`self.K2_GetPawn`)))
      (bind _patrolpoint (`/Game/NPCs/Enemies/BP_EnemyBaseCharacter.GetCurrentPatrolTarget` _asbp_enemy_base_character))
      (bind _key (`/Game/Utils/BPFL_BlackboardKeyNames.TargetPatrolPointKey`))
      (`BlackboardComponent.SetValueAsObject` _blackboardcomponent _key _patrolpoint)
      (else
        (`/Game/Utils/BPFL_Logging.Error` self "Failed to initialize behavior tree!" "InitializeBehaviorTree")))
    (else
      (`/Game/Utils/BPFL_Logging.Error` self "Failed to initialize behavior tree!" "InitializeBehaviorTree"))))

(fn `UpdateHasTarget`
  (params (SensedActor :type "Actor Object Reference") (HasTarget :type Boolean))
  (bind _returnvalue (`AIBlueprintHelperLibrary.GetBlackboard` null))
  (bind _asbp_first_person_character (cast `/Game/FirstPerson/Blueprints/BP_FirstPersonCharacter` SensedActor))
  (bind _key (`/Game/Utils/BPFL_BlackboardKeyNames.TargetActorKey`))
  (`BlackboardComponent.SetValueAsObject` _returnvalue _key _asbp_first_person_character)
  (bind _key_2 (`/Game/Utils/BPFL_BlackboardKeyNames.HasTargetKey`))
  (`BlackboardComponent.SetValueAsBool` _returnvalue _key_2 HasTarget))

(fn `UserConstructionScript`)