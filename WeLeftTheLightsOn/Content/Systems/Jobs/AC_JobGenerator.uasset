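; Actor component that procedurally generates randomized jobs from data tables, each with an energy cost and money-rewarded objectives.
; It picks random job templates, then builds one mandatory objective plus additional, randomly optional ones from each template's allowed types.
; Fetch and recovery or resource gathering objectives draw target items from item data filtered by type.
; Per-placeholder resolvers fill brace-delimited tokens in titles and descriptions, which are then capitalized.
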(fn `GenerateJob`
  (params (JobData :type "/Game/Systems/Jobs/Data/ST_JobData Structure"))
  (returns (Job :type "/Game/Systems/Jobs/JobStructs/ST_Job Structure"))
  (locals (Objectives :type "Array of /Game/Systems/Jobs/JobStructs/ST_Objective Structure"))
  (bind (_title _description _possibleobjectives _resolver) (break `/Game/Systems/Jobs/Data/ST_JobData` JobData))
  ; Initial "main" objective
  (bind _objective (`self.GenerateObjective` true _possibleobjectives))
  (`KismetArrayLibrary.Array_Add` (`local.Objectives`) _objective)
  ; Additional objectives
  (for _ (range 1 (+ (`self.MaxAdditionalObjectives`) 1))
    (bind _objective_2 (`self.GenerateObjective` false _possibleobjectives))
    (`KismetArrayLibrary.Array_Add` (`local.Objectives`) _objective_2))
  (bind _resolvedjob (`self.GenerateTitleAndDescription` (make `/Game/Systems/Jobs/JobStructs/ST_Job` _title _description (`KismetMathLibrary.RandomIntegerInRange` (`self.MinCost`) (`self.MaxCost`)) (`local.Objectives`) (`KismetStringLibrary.Conv_StringToName` (`KismetGuidLibrary.Conv_GuidToString` (`KismetGuidLibrary.NewGuid`)))) _resolver))
  (return _resolvedjob))

(fn `GenerateJobs`
  (params (Amount :type Integer))
  (returns (Jobs :type "Array of /Game/Systems/Jobs/JobStructs/ST_Job Structure"))
  (locals (GeneratedJobs :type "Array of /Game/Systems/Jobs/JobStructs/ST_Job Structure"))
  (bind _jobdata (`self.SelectRandomJobData` Amount))
  (for _array_element _jobdata
    (bind _job (`self.GenerateJob` _array_element))
    (`KismetArrayLibrary.Array_Add` (`local.GeneratedJobs`) _job))
  (return (`local.GeneratedJobs`)))

(fn `GenerateObjective`
  (params (ForceMandatory :type Boolean) (ObjectiveTypes :type "Array of /Game/Systems/Jobs/EN_ObjectiveType Enum"))
  (returns (Objective :type "/Game/Systems/Jobs/JobStructs/ST_Objective Structure"))
  (locals (ObjectiveItemTypes :type "Array of /Game/Systems/Items/Data/EN_ItemType Enum") (ObjectiveType :type "/Game/Systems/Jobs/EN_ObjectiveType Enum") (ObjectiveItemAmount :type Integer) (FilteredRowNames :type "Array of Name") (ObjectiveItem :type Name))
  (bind _objectiveitemtypes (`local.ObjectiveItemTypes`))
  (bind _output_get (set `local.ObjectiveType` (`KismetArrayLibrary.Array_Random` ObjectiveTypes)))
  ; Determine viable item types and amounts for objectives (Handle with caching)
  (switch `/Game/Systems/Jobs/EN_ObjectiveType` _output_get
    (:`NewEnumerator0`
      (`KismetArrayLibrary.Array_Append` _objectiveitemtypes (`|MakeArray` "NewEnumerator2" "NewEnumerator3" "NewEnumerator4" "NewEnumerator5" "NewEnumerator6" :!type "/Game/Systems/Items/Data/EN_ItemType Enum"))
      (set `local.ObjectiveItemAmount` 1))
    (:`NewEnumerator3`
      (`KismetArrayLibrary.Array_Add` _objectiveitemtypes "NewEnumerator0")
      (set `local.ObjectiveItemAmount` (`KismetMathLibrary.RandomIntegerInRange` 5 30))))
  ; Filter items by viable types for objective type (Handle with caching)
  (bind _outrownames (`DataTableFunctionLibrary.GetDataTableRowNames` "/Game/Systems/Items/Data/DT_ItemData.DT_ItemData"))
  (for _array_element _outrownames
    (bind _returnvalue (`|GetDataTableRow` "/Game/Systems/Items/Data/DT_ItemData.DT_ItemData" _array_element)
      (:`then`
        (if (`KismetArrayLibrary.Array_Contains` (`local.ObjectiveItemTypes`) (`.Type_9_15405C6C4AC7215D8FA4B8BDC52D0A4D` (break `/Game/Systems/Items/Data/ST_ItemData` _returnvalue)))
          (`KismetArrayLibrary.Array_Add` (`local.FilteredRowNames`) _array_element)))))
  ; Construct objective
  (bind _output_get_2 (set `local.ObjectiveItem` (`KismetArrayLibrary.Array_Random` (`local.FilteredRowNames`))))
  (bind _returnvalue_2 (`|GetDataTableRow` "/Game/Systems/Items/Data/DT_ItemData.DT_ItemData" _output_get_2)
    (:`then`
      (bind (_type _name _maxquantity _definition) (break `/Game/Systems/Items/Data/ST_ItemData` _returnvalue_2))
      (return (make `/Game/Systems/Jobs/JobStructs/ST_Objective` _name (`/Game/Systems/Items/Data/DA_ItemDefinition.Description` _definition) (`local.ObjectiveType`) (make `/Game/Systems/Jobs/JobStructs/ST_Reward` (`KismetMathLibrary.RandomIntegerInRange` (`self.MinReward`) (`self.MaxReward`))) (select `bool` (`local.ForceMandatory`) :`false` (`KismetMathLibrary.RandomBool`)) (make `/Game/Systems/Jobs/JobStructs/ST_CompletionDetails` false _output_get_2 (`local.ObjectiveItemAmount`)))))))

(fn `GenerateTitleAndDescription`
  (params (Job :type "/Game/Systems/Jobs/JobStructs/ST_Job Structure") (Resolver :type "Array of /Game/Systems/Jobs/Data/Resolver/DA_JobTextResolver Object Reference"))
  (returns (ResolvedJob :type "/Game/Systems/Jobs/JobStructs/ST_Job Structure (by ref)"))
  (locals (TitleInProgress :type String) (DesriptionInProgress :type String) (PlaceholderToResolver :type "Map of /Game/Systems/Jobs/Data/EN_JobPlaceholders Enum to /Game/Systems/Jobs/Data/Resolver/DA_JobTextResolver Object Reference"))
  (bind (_title _description) (break `/Game/Systems/Jobs/JobStructs/ST_Job` Job))
  (set `local.TitleInProgress` (`KismetTextLibrary.Conv_TextToString` _title))
  (set `local.DesriptionInProgress` (`KismetTextLibrary.Conv_TextToString` _description))
  (for _array_element Resolver
    ; Build quick resolver lookup (Rework into a cache)
    (for _array_element_2 (`/Game/Systems/Jobs/Data/Resolver/DA_JobTextResolver.Placeholder` _array_element)
      (`BlueprintMapLibrary.Map_Add` (`local.PlaceholderToResolver`) _array_element_2 _array_element)))
  ; Resolve placeholder
  (bind _enumvalue (foreach `/Game/Systems/Jobs/Data/EN_JobPlaceholders` false)
    (:`LoopBody`
      (bind (_value _returnvalue) (`BlueprintMapLibrary.Map_Find` (`local.PlaceholderToResolver`) _enumvalue))
      (if _returnvalue
        (bind _replacement (`/Game/Systems/Jobs/Data/Resolver/DA_JobTextResolver.Resolve` _value (`local.Job`) _enumvalue))
        ; Replace placeholders
        (bind _resolved (`self.ReplacePlaceholder` (`local.TitleInProgress`) _enumvalue _replacement))
        (set `local.TitleInProgress` _resolved)
        (bind _resolved_2 (`self.ReplacePlaceholder` (`local.DesriptionInProgress`) _enumvalue _replacement))
        (set `local.DesriptionInProgress` _resolved_2)))
    (:`then`
      ; Capitilize texts & update job
      (bind _string (`/Game/Utils/BPFL_Operations.CapitalizeString` (`local.TitleInProgress`)))
      (bind _string_2 (`/Game/Utils/BPFL_Operations.CapitalizeString` (`local.DesriptionInProgress`)))
      (bind _structout (setmembers `/Game/Systems/Jobs/JobStructs/ST_Job` :`StructRef` Job :`Title` (`KismetTextLibrary.Conv_StringToText` _string) :`Description` (`KismetTextLibrary.Conv_StringToText` _string_2)))
      (return _structout))))

(fn `ReplacePlaceholder`
  (params (Source :type String) (Placeholder :type "/Game/Systems/Jobs/Data/EN_JobPlaceholders Enum" :default "NewEnumerator0") (Replacement :type String))
  (returns (Resolved :type String))
  (return (`KismetStringLibrary.Replace` Source (`KismetStringLibrary.Concat_StrStr` (`KismetStringLibrary.Concat_StrStr` "{" (`|GetEnumeratorNameAsString` Placeholder)) "}") Replacement)))

(fn `SelectRandomJobData`
  (params (Amount :type Integer))
  (returns (JobData :type "Array of /Game/Systems/Jobs/Data/ST_JobData Structure"))
  (locals (SelectedJobs :type "Array of /Game/Systems/Jobs/Data/ST_JobData Structure"))
  (bind _outrownames (`DataTableFunctionLibrary.GetDataTableRowNames` "/Game/Systems/Jobs/Data/DT_JobData.DT_JobData"))
  (for _ (range 1 (+ Amount 1))
    (bind _returnvalue (`|GetDataTableRow` "/Game/Systems/Jobs/Data/DT_JobData.DT_JobData" (`KismetArrayLibrary.Array_Random` _outrownames))
      (:`then`
        (`KismetArrayLibrary.Array_Add` (`local.SelectedJobs`) _returnvalue))))
  (return (`local.SelectedJobs`)))