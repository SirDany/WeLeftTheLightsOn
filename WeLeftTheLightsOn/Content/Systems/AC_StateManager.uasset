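; State manager component that gives its owner access to the shared ship and job states.
; Getter and updater functions cast the current GameState to BP_GameStateBase and forward each call to it, so the component stores no state itself.
; Each function returns a success flag and logs an error with the function name when the cast fails.
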(fn `GetJobState`
  (returns (JobState :type "/Game/Systems/Jobs/ST_JobState Structure") (Success :type Boolean))
  (bind _asbp_game_state_base (cast `/Game/Systems/BP_GameStateBase` (`GameplayStatics.GetGameState`))
    (:`then`
      (bind _jobstate (`/Game/Systems/BP_GameStateBase.GetJobState` _asbp_game_state_base))
      (return _jobstate true))
    (:`CastFailed`
      (`/Game/Utils/BPFL_Logging.Error` self "Could not retrieve GameState." "GetJobState")
      (return (struct) false))))

(fn `GetShipState`
  (returns (ShipState :type "/Game/Systems/Ship/ST_ShipState Structure") (Success :type Boolean))
  (bind _asbp_game_state_base (cast `/Game/Systems/BP_GameStateBase` (`GameplayStatics.GetGameState`))
    (:`then`
      (bind _shipstate (`/Game/Systems/BP_GameStateBase.GetShipState` _asbp_game_state_base))
      (return _shipstate true))
    (:`CastFailed`
      (`/Game/Utils/BPFL_Logging.Error` self "Could not retrieve GameState." "GetShipState")
      (return (struct) false))))

(fn `UpdateJobState`
  (params (JobState :type "/Game/Systems/Jobs/ST_JobState Structure"))
  (returns (Success :type Boolean))
  (bind _asbp_game_state_base (cast `/Game/Systems/BP_GameStateBase` (`GameplayStatics.GetGameState`))
    (:`then`
      (`/Game/Systems/BP_GameStateBase.UpdateJobState` _asbp_game_state_base JobState)
      (return true))
    (:`CastFailed`
      (`/Game/Utils/BPFL_Logging.Error` self "Could not retrieve GameState." "UpdateJobState")
      (return false))))

(fn `UpdateShipState`
  (params (ShipState :type "/Game/Systems/Ship/ST_ShipState Structure"))
  (returns (Success :type Boolean))
  (bind _asbp_game_state_base (cast `/Game/Systems/BP_GameStateBase` (`GameplayStatics.GetGameState`))
    (:`then`
      (`/Game/Systems/BP_GameStateBase.UpdateShipState` _asbp_game_state_base ShipState)
      (return true))
    (:`CastFailed`
      (`/Game/Utils/BPFL_Logging.Error` null "Could not retrieve GameState." "UpdateShipState")
      (return false))))