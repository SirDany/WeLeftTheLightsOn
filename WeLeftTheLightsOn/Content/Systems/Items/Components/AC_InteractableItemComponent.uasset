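; AC_InteractableItemComponent is an item interaction component that defines which inputs a BP_Item responds to in its current state.
; A nested map keyed by ItemState, then input, supplies each interaction's description and sound.
; GetAvailableInteractions substitutes the DT_ItemData name into description placeholders, and CanHandleInput checks inputs against that result.
; Interact is a stub here, returning RemoveInteractable as false.
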(fn `CanHandleInput`
  (params (Input :type "InputAction Object Reference"))
  (returns (CanHandle :type Boolean))
  (bind _interactions (`self.GetAvailableInteractions`))
  (return (`BlueprintMapLibrary.Map_Contains` _interactions Input)))

(fn `GetAvailableInteractions`
  (returns (Interactions :type "Map of InputAction Object Reference to Text"))
  (locals (ReplacedInteractions :type "Map of InputAction Object Reference to Text") (ItemNamePlaceHolder :type String :default "{item}"))
  ; Find interactions based on item state
  (bind _asbp_item (cast `/Game/Systems/Items/Blueprints/BP_Item` (`self.GetOwner`))
    (:`then`
      (bind (_value _returnvalue) (`BlueprintMapLibrary.Map_Find` (`self.Interactions`) (`/Game/Systems/Items/Blueprints/BP_Item.ItemState` _asbp_item)))
      (if _returnvalue
        ; Replace item name placeholders
        (bind _returnvalue_2 (`|GetDataTableRow` "/Game/Systems/Items/Data/DT_ItemData.DT_ItemData" (`/Game/Systems/Items/Blueprints/BP_Item.ID` _asbp_item))
          (:`then`
            (bind (_keypin _valuepin) (`|MapForEach` (`.Interactions_9_CC4C975942DA7FA1500F15A91A85F114` (break `/Game/Systems/Items/Components/ST_ItemInteractionsMap` _value)))
              (:`then`
                (`BlueprintMapLibrary.Map_Add` (`local.ReplacedInteractions`) _keypin (`KismetTextLibrary.Conv_StringToText` (`KismetStringLibrary.Replace` (`KismetTextLibrary.Conv_TextToString` (`.Description_8_CC4C975942DA7FA1500F15A91A85F114` (break `/Game/Systems/Items/Components/ST_ItemInteractionsMapValue` _valuepin))) (`local.ItemNamePlaceHolder`) (`KismetTextLibrary.Conv_TextToString` (`.Name_23_E77874D9448027E501115793B2E741C2` (break `/Game/Systems/Items/Data/ST_ItemData` _returnvalue_2)))))))
              (:`CompletedPin`
                (return (`local.ReplacedInteractions`))))))
        (else
          (return))))
    (:`CastFailed`
      (return))))

(fn `GetInteractionSound`
  (params (Input :type "InputAction Object Reference"))
  (returns (Sound :type "SoundBase Object Reference"))
  (bind _asbp_item (cast `/Game/Systems/Items/Blueprints/BP_Item` (`self.GetOwner`)))
  (bind (_value _returnvalue) (`BlueprintMapLibrary.Map_Find` (`self.Interactions`) (`/Game/Systems/Items/Blueprints/BP_Item.ItemState` _asbp_item)))
  (if _returnvalue
    (bind (_value_2 _returnvalue_2) (`BlueprintMapLibrary.Map_Find` (`.Interactions_9_CC4C975942DA7FA1500F15A91A85F114` (break `/Game/Systems/Items/Components/ST_ItemInteractionsMap` _value)) Input))
    (if _returnvalue_2
      (return (`.Sound_11_A6CFF28045C7D8EF9BCC4F9FD5B682E4` (break `/Game/Systems/Items/Components/ST_ItemInteractionsMapValue` _value_2))))))

(fn `Interact`
  (params (Controller :type "Controller Object Reference") (Input :type "InputAction Object Reference"))
  (returns (RemoveInteractable :type Boolean) (PlaySound :type "SoundBase Object Reference"))
  (return false null))