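; AC_Consume is an item behavior component that lets a player controller consume the world BP_Item it is attached to.
; RenderItem applies the world mesh and relative transform from the owner's ItemDefinition.
; Interact checks that it can handle the input, then passes the item ID to the controller's ConsumeItemMessage.
; On success it flags the interactable for removal and returns the interaction sound for that input.
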(event `self.ReceiveBeginPlay`)

(fn `Interact`
  (params (Controller :type "Controller Object Reference") (Input :type "InputAction Object Reference"))
  (returns (RemoveInteractable :type Boolean) (PlaySound :type "SoundBase Object Reference"))
  (bind _canhandle (`self.CanHandleInput` Input))
  (if _canhandle
    (bind _asbp_item (cast `/Game/Systems/Items/Blueprints/BP_Item` (`self.GetOwner`)))
    (bind _success (message `/Game/Systems/Items/Blueprints/BPI_ItemInteractionReceiver.ConsumeItem` Controller (`/Game/Systems/Items/Blueprints/BP_Item.ID` _asbp_item)))
    (if _success
      (bind _sound (`self.GetInteractionSound` Input))
      (return true _sound))))

(fn `RenderItem`
  (params (Mesh :type "StaticMeshComponent Object Reference"))
  (bind _asbp_item (cast `/Game/Systems/Items/Blueprints/BP_Item` (`self.GetOwner`)))
  (bind _itemdefinition (`/Game/Systems/Items/Blueprints/BP_Item.ItemDefinition` _asbp_item))
  (`StaticMeshComponent.SetStaticMesh` Mesh (`/Game/Systems/Items/Data/DA_ItemDefinition.WorldMesh` _itemdefinition))
  (`SceneComponent.K2_SetRelativeTransform` Mesh (`/Game/Systems/Items/Data/DA_ItemDefinition.WorldTransform` _itemdefinition) false false))