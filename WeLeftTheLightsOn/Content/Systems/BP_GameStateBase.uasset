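; Game state Blueprint that holds the current job state and ship state and notifies listeners when they change.
; UpdateJobState and UpdateShipState store the incoming state and call the matching update dispatcher, with getters exposing both values.
; UpdateJobState also checks HasActiveJob before overwriting, intended to announce a newly active job through OnActiveJobSet.
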(event `self.ReceiveBeginPlay`)

(fn `GetJobState`
  (returns (JobState :type "/Game/Systems/Jobs/ST_JobState Structure"))
  (return (`self.JobState`)))

(fn `GetShipState`
  (returns (ShipState :type "/Game/Systems/Ship/ST_ShipState Structure"))
  (return (`self.ShipState`)))

(fn `UpdateJobState`
  (params (JobState :type "/Game/Systems/Jobs/ST_JobState Structure"))
  (locals (NewActiveJobSet :type Boolean))
  (bind (_activejob _availablejobs _hasactivejob) (break `/Game/Systems/Jobs/ST_JobState` JobState))
  (set `local.NewActiveJobSet` (and _hasactivejob (not (`.HasActiveJob_13_0208072C43EEBF76856A8C91F30FADC0` (break `/Game/Systems/Jobs/ST_JobState` (`self.JobState`))))))
  (bind _output_get (set `self.JobState` JobState))
  (`self.OnJobStateUpdated` _output_get)
  (if (`local.NewActiveJobSet`)
    (`self.OnActiveJobSet` _activejob)))

(fn `UpdateShipState`
  (params (ShipState :type "/Game/Systems/Ship/ST_ShipState Structure"))
  (bind _output_get (set `self.ShipState` ShipState))
  (`self.OnShipStateUpdated` _output_get))

(fn `UserConstructionScript`)