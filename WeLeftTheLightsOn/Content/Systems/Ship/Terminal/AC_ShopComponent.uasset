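; Shop component for the ship terminal system that lets credits be traded for ship energy.
; BuyEnergy fetches the ship state, checks Money against the requested amount, then moves that amount from Money to Energy at a one-to-one rate and writes it back.
; It returns the resulting state and a success flag, warning when credits are short.
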(fn `BuyEnergy`
  (params (`Amount to buy` :type Integer))
  (returns (CurrentShipState :type "/Game/Systems/Ship/ST_ShipState Structure") (Success :type Boolean))
  (bind (_shipstate _success) (`self.GetShipState`))
  (if _success
    (bind (_energy _money) (break `/Game/Systems/Ship/ST_ShipState` _shipstate))
    (if (>= _money `Amount to buy`)
      (bind _structout (setmembers `/Game/Systems/Ship/ST_ShipState` :`StructRef` _shipstate :`Energy` (+ _energy `Amount to buy`) :`Money` (- _money `Amount to buy`)))
      (bind _success_2 (`self.UpdateShipState` _structout))
      (return _structout _success_2)
      (else
        (`/Game/Utils/BPFL_Logging.Warn` self "Not enough Credits!" "BuyEnergy")
        (return _shipstate false)))))