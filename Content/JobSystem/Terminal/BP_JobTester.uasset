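; BP_JobTester is a debug Blueprint that exercises random job generation in the job system.
; On BeginPlay it repeatedly calls GenerateRandomJob with its ObjectiveTypes, a fixed tier and optional objectives enabled.
; Each job's objectives are formatted into text lines with reward, type and optional state, then joined under the job's title, description and energy cost and printed through PrintString.
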(event `self.ReceiveBeginPlay`
  (for _ (range 3)
    (`KismetArrayLibrary.Array_Clear` (`self.FormattedObjectiveStrings`))
    (bind _job (`/Game/JobSystem/BPFL_JobGeneration.GenerateRandomJob` (`self.ObjectiveTypes`) 1.0 true))
    (bind (_jobtitle _jobdescription _energycost _objectives) (break `/Game/JobSystem/FJob` _job))
    (for _array_element _objectives
      (bind (_objectivetitle _objectivedescription _objectivetype _reward _isoptional) (break `/Game/JobSystem/FObjective` _array_element))
      (`KismetArrayLibrary.Array_Add` (`self.FormattedObjectiveStrings`) (`KismetTextLibrary.Conv_TextToString` (`|FormatText` "- {Title}: {Desc} (Reward: {Reward} Credits), Type: {Type}, {OptionalState}" _objectivetitle _objectivedescription _reward (`|GenericToText` _objectivetype) (`KismetMathLibrary.SelectText` "Optional" "Mandatory" _isoptional)))))
    (`KismetSystemLibrary.PrintString` (`KismetStringLibrary.Concat_StrStr` (`KismetTextLibrary.Conv_TextToString` (`|FormatText` " \nJob: {JobTitle} \n{JobDesc} \nCost: {Cost} Credits \nObjectives: \n" _jobtitle _jobdescription _energycost)) (`KismetStringLibrary.JoinStringArray` (`self.FormattedObjectiveStrings`) "\\n ")))))

(fn `UserConstructionScript`)