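; BP_JobTester is a debug Blueprint that exercises the job system when play begins.
; It generates three jobs from its objective types, including optional objectives, prints each, then tries to set the first as active and reports the result.
; The PrintJob helper formats a job's title, description, energy cost and objectives, with credit rewards and optional or mandatory state, into one on-screen string.
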(event `self.ReceiveBeginPlay`
  (bind (_success _jobs) (`/Game/Systems/JobSystem/BPFL_JobManager.GenerateAvailableJobs` (`self.ObjectiveTypes`) 1.0 true 3))
  (for _array_element _jobs
    (`self.PrintJob` _array_element))
  (bind _output (`|GetArrayItem` _jobs))
  (bind _success_2 (`/Game/Systems/JobSystem/BPFL_JobManager.SetActiveJob` _output))
  (if _success_2
    (`KismetSystemLibrary.PrintText` "Selected Job: ")
    (`self.PrintJob` _output)
    (else
      (`KismetSystemLibrary.PrintText` "Unable to select job!" true true (struct :`R` 1.0 :`G` 0.035601 :`A` 1.0)))))

(fn `PrintJob`
  (params (Job :type "/Game/Systems/JobSystem/JobStructs/ST_Job Structure"))
  (locals (FormattedObjectiveStrings :type "Array of String") (Divider :type Text :default "NSLOCTEXT(\"[7F4DFD0FBB275CEFB0ACA88B9B255100]\", \"F2155E924882D0A5FAD4829F0616928F\", \"====================================================================================================================================================================================================\")"))
  (bind (_jobtitle _jobdescription _energycost _objectives) (break `/Game/Systems/JobSystem/JobStructs/ST_Job` Job))
  (for _array_element _objectives
    (bind (_objectivetitle _objectivedescription _objectivetype _reward _isoptional) (break `/Game/Systems/JobSystem/JobStructs/ST_Objective` _array_element))
    (`KismetArrayLibrary.Array_Add` (`local.FormattedObjectiveStrings`) (`KismetTextLibrary.Conv_TextToString` (`|FormatText` "- {Title}: {Desc} (Reward: {Reward} Credits), Type: {Type}, {OptionalState}" _objectivetitle _objectivedescription (`.Money_2_AFA861594D57F02B5B5D77BABEF9E904` (break `/Game/Systems/JobSystem/JobStructs/ST_Reward` _reward)) (`|GenericToText` _objectivetype) (`KismetMathLibrary.SelectText` "Optional" "Mandatory" _isoptional)))))
  (`KismetSystemLibrary.PrintString` (`KismetTextLibrary.Conv_TextToString` (`|FormatText` " \n{Divider} \nJob: {JobTitle} \n{JobDesc} \nCost: {Cost} Energy \nObjectives: \n{Objectives} \n{Divider}" (`local.Divider`) _jobtitle _jobdescription _energycost (`KismetStringLibrary.JoinStringArray` (`local.FormattedObjectiveStrings`) "\\n ")))))

(fn `UserConstructionScript`)