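; Base hazard actor for a proximity-triggered explosion, configured from a hazard data table row by ID.
; On BeginPlay the row sets the trigger sphere's radius and fuse time; any overlap starts the timer, and any end overlap cancels it.
; Explode enables physics on a Geometry Collection, plays a sound and applies an upward impulse.
; Player damage is a placeholder distance check that only prints.
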(event `self.ReceiveBeginPlay`
  (`self.Initialize`))

(event `self.Sphere.OnComponentBeginOverlap`
  (params (OverlappedComponent :type "PrimitiveComponent Object Reference") (OtherActor :type "Actor Object Reference") (OtherComp :type "PrimitiveComponent Object Reference") (OtherBodyIndex :type Integer) (bFromSweep :type Boolean) (SweepResult :type "HitResult Structure (by ref)"))
  (bind _returnvalue (`KismetSystemLibrary.K2_SetTimer` null "Explode" (`self.Trigger Timer`)))
  (set `self.Timer` _returnvalue)
  (bind _asbp_first_person_character (cast `/Game/FirstPerson/Blueprints/BP_FirstPersonCharacter` OtherActor))
  (set `self.As BP First Person Character` _asbp_first_person_character))

(event `self.Sphere.OnComponentEndOverlap`
  (params (OverlappedComponent :type "PrimitiveComponent Object Reference") (OtherActor :type "Actor Object Reference") (OtherComp :type "PrimitiveComponent Object Reference") (OtherBodyIndex :type Integer))
  (`KismetSystemLibrary.K2_ClearAndInvalidateTimerHandle` (`self.Timer`))
  (set `self.As BP First Person Character` null))

(fn `Explode`
  (`PrimitiveComponent.SetSimulatePhysics` (`self.GC_FractureComponent`) true)
  (`GameplayStatics.PlaySoundAtLocation` (`self.sound`) (`self.K2_GetActorLocation`) (struct) 1.0 1.0 0.0 null null null null)
  (`PrimitiveComponent.AddImpulse` (`self.GC_FractureComponent`) (0.0 0.0 100000.0) "None" false)
  (if (`KismetSystemLibrary.IsValid` (`self.As BP First Person Character`))
    ; Apply damage or debuffs here. Needs rework in combination with Hazard data
    (if (<= (`self.GetDistanceTo` (`self.As BP First Person Character`) self) 100.0)
      (`KismetSystemLibrary.PrintString` "Player took damage"))))

(fn `Initialize`
  (locals (TriggerTimer :type "Float (double-precision)"))
  (bind _returnvalue (`|GetDataTableRow` (`self.DataTable`) (`self.ID`))
    (:`then`
      (bind (_name _description _damage _triggerradius _triggertimer) (break `/Game/Systems/Hazards/Data/ST_HazardData` _returnvalue))
      (`SphereComponent.SetSphereRadius` (`self.Sphere`) _triggerradius true)
      (set `self.Trigger Timer` _triggertimer))
    (:`RowNotFound`
      (`KismetSystemLibrary.PrintString` "Hazard not found in Hazard data table"))))

(fn `UserConstructionScript`)