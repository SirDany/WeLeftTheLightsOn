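; Pickupable world item that the player collects by pressing E while inside its sphere collider.
; Overlap shows the prompt widget, enables input and caches the player; leaving hides the prompt and disables input.
; E sends the item to the player through PickupItemMessage, then notifies BP_GameStateBase on success.
; Update refreshes the prompt with the item name, while a work-in-progress GameState inventory function remains unused in the event graph.
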(event `Key|E`
  (params (Key :type "Key Structure"))
  (bind _id (`self.ID`))
  ; Move to player Controller
  (:`Pressed`
    (bind _success (message `/Game/Systems/Item/Blueprints/BPI_Pickupable.PickupItem` (`self.Player`) (`self.ID`) (`self.Item`) self))
    (if _success
      ; Needs to be reworked
      (bind _asbp_game_state_base (cast `/Game/Systems/BP_GameStateBase` (`GameplayStatics.GetGameState`))
        (:`then`
          (`/Game/Systems/BP_GameStateBase.OnItemPickup` _asbp_game_state_base _id 1))
        (:`CastFailed`
          (`/Game/Utils/BPFL_Logging.Error` self (`|FormatText` "Failed to notify GameState about item pickup with itemID: {id}." _id) "OnBeginComponentOverlap"))))))

(event `self.ReceiveBeginPlay`
  ; Calls the item replication function when pickup starts
  (`parent.ReceiveBeginPlay`)
  (`self.InitializePickupItem`))

(event `Update`
  ; Updates the item mesh when it is picked up and activates interact widget
  (bind _aswbp_pickup (cast `/Game/Systems/Item/Widgets/WBP_Pickup` (`WidgetComponent.GetWidget` (`self.ItemPickupPrompt`))))
  (`/Game/Systems/Item/Widgets/WBP_Pickup.UpdateActionPrompt` _aswbp_pickup (`.Name_23_E77874D9448027E501115793B2E741C2` (break `/Game/Systems/Item/Data/ST_ItemData` (`self.Item`))))
  (`parent.Update`))

(event `self.SphereComponent.OnComponentBeginOverlap`
  (params (OverlappedComponent :type "PrimitiveComponent Object Reference") (OtherActor :type "Actor Object Reference") (OtherComp :type "PrimitiveComponent Object Reference") (OtherBodyIndex :type Integer) (bFromSweep :type Boolean) (SweepResult :type "HitResult Structure (by ref)"))
  ; Enable interactions on item upon entering collision zone
  (bind _ascharacter (cast `Character` OtherActor))
  (bind _isplayer (`/Game/Utils/BPFL_InteractUtils.IsPlayer` _ascharacter))
  (if _isplayer
    (`SceneComponent.SetVisibility` (`self.ItemPickupPrompt`) true false)
    (`self.EnableInput` (`GameplayStatics.GetPlayerController` 0))
    (set `self.Player` _ascharacter)))

(event `self.SphereComponent.OnComponentEndOverlap`
  (params (OverlappedComponent :type "PrimitiveComponent Object Reference") (OtherActor :type "Actor Object Reference") (OtherComp :type "PrimitiveComponent Object Reference") (OtherBodyIndex :type Integer))
  ; Disables interaction on Item when leaving collision zone
  (bind _ascharacter (cast `Character` OtherActor))
  (bind _isplayer (`/Game/Utils/BPFL_InteractUtils.IsPlayer` _ascharacter))
  (if _isplayer
    (`SceneComponent.SetVisibility` (`self.ItemPickupPrompt`) false false)
    (`self.DisableInput` (`GameplayStatics.GetPlayerController` 0))))

(fn `AddToInventory_WIP`
  (locals (FoundInventoryIndex_WIP :type Integer :default -1))
  (bind _id (`self.ID`))
  (bind _foundinventoryindex_wip (`local.FoundInventoryIndex_WIP`))
  (bind _returnvalue (>= _foundinventoryindex_wip 0))
  (bind _asbp_game_state_base (cast `/Game/Systems/BP_GameStateBase` (`GameplayStatics.GetGameState`))
    (:`then`
      (bind _inventory_wip (`/Game/Systems/BP_GameStateBase.Inventory_WIP` _asbp_game_state_base))
      (for (_array_element _array_index) _inventory_wip
        (if (== (`.PickupItemID_2_3E965EB4449FE3267E33A3BF34BC489A` (break `/Game/Systems/ST_InventorySlot_WIP` _array_element)) _id)
          (set `local.FoundInventoryIndex_WIP` _array_index)
          (break)))
      (if _returnvalue
        (bind _returnvalue_2 (`KismetMathLibrary.SelectInt` (+ (`.Amount_5_78C76B7942B6B4EB598E6AB1AFB82BD2` (break `/Game/Systems/ST_InventorySlot_WIP` (`|GetArrayItem` _inventory_wip _foundinventoryindex_wip))) 1) 1 _returnvalue))
        (bind _st_inventoryslot_wip (make `/Game/Systems/ST_InventorySlot_WIP` _id _returnvalue_2))
        (`KismetArrayLibrary.Array_Set` _inventory_wip _foundinventoryindex_wip _st_inventoryslot_wip _returnvalue)
        (else
          (`KismetArrayLibrary.Array_Add` _inventory_wip _st_inventoryslot_wip)))
      (`/Game/Utils/BPFL_Logging.Info` self (`|FormatText` "{Action} | ItemID: {ID} | Amount {Amount}" (`KismetMathLibrary.SelectText` "Updated item in inventory." "Added item to inventory." _returnvalue) _id _returnvalue_2) "AddToInventory_WIP"))
    (:`CastFailed`
      (`/Game/Utils/BPFL_Logging.Warn` self "Failed to get GameState." "AddToInventory_WIP"))))

(fn `InitializePickupItem`
  (bind _spherecomponent (`self.SphereComponent`))
  (`PrimitiveComponent.SetCollisionEnabled` _spherecomponent "QueryOnly")
  (`SceneComponent.SetVisibility` _spherecomponent false false))

(fn `UserConstructionScript`)