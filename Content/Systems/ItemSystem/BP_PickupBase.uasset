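; Base pickup actor for world items that the first-person character collects by overlapping its sphere.
; The construction script looks up its ID in an item data table to set the world mesh and collision, warning if no row exists.
; On overlap it hides the mesh and disables collision without destroying the actor.
; A temporary WIP function then increments or adds that item's slot in the GameState inventory array and logs the result.
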(event `self.SphereComponent.OnComponentBeginOverlap`
  (params (OverlappedComponent :type "PrimitiveComponent Object Reference") (OtherActor :type "Actor Object Reference") (OtherComp :type "PrimitiveComponent Object Reference") (OtherBodyIndex :type Integer) (bFromSweep :type Boolean) (SweepResult :type "HitResult Structure (by ref)"))
  (bind _pickupmeshcomponent (`self.PickupMeshComponent`))
  (cast `/Game/FirstPerson/Blueprints/BP_FirstPersonCharacter` OtherActor)
  (`SceneComponent.SetVisibility` _pickupmeshcomponent false false)
  (`PrimitiveComponent.SetCollisionEnabled` _pickupmeshcomponent "NoCollision")
  (`PrimitiveComponent.SetCollisionEnabled` (`self.SphereComponent`) "NoCollision")
  (`self.AddToInventory_WIP` :!pinned true) ; Remove this when implementing proper inventory
)

(fn `AddToInventory_WIP`
  (locals (FoundInventoryIndex_WIP :type Integer :default -1))
  (bind _id (`self.ID`))
  (bind _foundinventoryindex_wip (`local.FoundInventoryIndex_WIP`))
  (bind _returnvalue (>= _foundinventoryindex_wip 0))
  (bind _asbp_game_state_base (cast `/Game/Systems/BP_GameStateBase` (`GameplayStatics.GetGameState`))
    (:`then`
      (bind _inventory_wip (`/Game/Systems/BP_GameStateBase.Inventory_WIP` _asbp_game_state_base))
      (for (_array_element _array_index) _inventory_wip
        (if (== (`.PickupItemID_2_3E965EB4449FE3267E33A3BF34BC489A` (break `/Game/Systems/ST_InventorySlot_WIP` _array_element)) _id)
          (set `local.FoundInventoryIndex_WIP` _array_index)
          (break)))
      (if _returnvalue
        (bind _returnvalue_2 (`KismetMathLibrary.SelectInt` (+ (`.Amount_5_78C76B7942B6B4EB598E6AB1AFB82BD2` (break `/Game/Systems/ST_InventorySlot_WIP` (`|GetArrayItem` _inventory_wip _foundinventoryindex_wip))) 1) 1 _returnvalue))
        (bind _st_inventoryslot_wip (make `/Game/Systems/ST_InventorySlot_WIP` _id _returnvalue_2))
        (`KismetArrayLibrary.Array_Set` _inventory_wip _foundinventoryindex_wip _st_inventoryslot_wip _returnvalue)
        (else
          (`KismetArrayLibrary.Array_Add` _inventory_wip _st_inventoryslot_wip)))
      (`/Game/Utils/BPFL_Logging.Info` self (`|FormatText` "{Action} | ItemID: {ID} | Amount {Amount}" (`KismetMathLibrary.SelectText` "Updated item in inventory." "Added item to inventory." _returnvalue) _id _returnvalue_2) "AddToInventory_WIP"))
    (:`CastFailed`
      (`/Game/Utils/BPFL_Logging.Warn` self "Failed to get GameState." "AddToInventory_WIP"))))

(fn `Initialize`
  (bind _id (`self.ID`))
  (bind _pickupmeshcomponent (`self.PickupMeshComponent`))
  (bind _spherecomponent (`self.SphereComponent`))
  (bind _output (`|ConvertAsset` (`self.ItemDataTable`)))
  (bind _returnvalue (`DataTableFunctionLibrary.DoesDataTableRowExist` _output _id))
  (if _returnvalue
    (bind _returnvalue_2 (`|GetDataTableRow` _output _id)
      (:`then`
        (bind _output_get (set `self.ReferenceItem` (`.Definition_11_8158F8FE468F141EE5B889BF9F2ED7B2` (break `/Game/Systems/ItemSystem/ST_ItemData` _returnvalue_2))))
        (`StaticMeshComponent.SetStaticMesh` _pickupmeshcomponent (`/Game/Systems/ItemSystem/DA_ItemDefinition.WorldMesh` _output_get))
        (`PrimitiveComponent.SetCollisionEnabled` _pickupmeshcomponent "NoCollision")
        (`PrimitiveComponent.SetCollisionEnabled` _spherecomponent "QueryOnly")
        (`SceneComponent.SetVisibility` _spherecomponent false false))
      (:`RowNotFound`
        (`/Game/Utils/BPFL_Logging.Warn` self (`|FormatText` "Unable to find row for item with ID: {id}" _id) "Initialize" :!label _label)))
    (else
      (goto _label))))

(fn `UserConstructionScript`
  (`self.Initialize`))