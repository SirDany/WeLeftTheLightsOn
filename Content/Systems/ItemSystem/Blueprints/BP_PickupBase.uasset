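; Base world pickup for an item ID, which a player collects by pressing E while in range.
; Construction and OnRep_ID, also called on BeginPlay, resolve data table rows into mesh and label, preferring dropped-item data.
; Sphere overlap toggles prompt and input for local non-AI characters and sets ownership for server-side destruction.
; A successful pickup message updates the placeholder GameState inventory, destroys the actor and notifies GameState.
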(event `DestroyOnServer`
  (`self.K2_DestroyActor`))

(event `Key|E`
  (params (Key :type "Key Structure"))
  (bind _id (`self.ID`))
  (:`Pressed`
    (bind _success (message `/Game/Systems/ItemSystem/Blueprints/BPI_PickupBase.PickupItem` (`self.Player`) (`self.ID`) (`self.Item`)))
    (if _success
      (`self.AddToInventory_WIP` :!pinned true) ; Remove this when implementing proper inventory
      (`self.DestroyOnServer`)
      ; Needs to be reworked
      (bind _asbp_game_state_base (cast `/Game/Systems/BP_GameStateBase` (`GameplayStatics.GetGameState`))
        (:`then`
          (`/Game/Systems/BP_GameStateBase.OnItemPickup` _asbp_game_state_base _id 1))
        (:`CastFailed`
          (`/Game/Utils/BPFL_Logging.Error` self (`|FormatText` "Failed to notify GameState about item pickup with itemID: {id}." _id) "OnBeginComponentOverlap"))))))

(event `self.ReceiveBeginPlay`
  ; Calls the item replication function when pickup starts
  (`self.OnRep_ID`))

(event `Update`
  (bind ((`Definition_11_8158F8FE468F141EE5B889BF9F2ED7B2` _definition) (`Name_23_E77874D9448027E501115793B2E741C2` _name)) (break `/Game/Systems/ItemSystem/Data/ST_ItemData` (`self.Item`)))
  ; Updates the item mesh when it is picked up
  (bind _aswbp_pickup (cast `/Game/Systems/ItemSystem/Widgets/WBP_Pickup` (`WidgetComponent.GetWidget` (`self.Widget`))))
  (`TextBlock.SetText` (`/Game/Systems/ItemSystem/Widgets/WBP_Pickup.Action` _aswbp_pickup) _name)
  (bind _returnvalue (`KismetSystemLibrary.LoadAsset_Blocking` (`|ConvertAsset` (`/Game/Systems/ItemSystem/Data/DA_ItemDefinition.WorldMesh` _definition))))
  (bind _asstatic_mesh (cast `StaticMesh` _returnvalue))
  (`StaticMeshComponent.SetStaticMesh` (`self.PickupMeshComponent`) _asstatic_mesh))

(event `self.SphereComponent.OnComponentBeginOverlap`
  (params (OverlappedComponent :type "PrimitiveComponent Object Reference") (OtherActor :type "Actor Object Reference") (OtherComp :type "PrimitiveComponent Object Reference") (OtherBodyIndex :type Integer) (bFromSweep :type Boolean) (SweepResult :type "HitResult Structure (by ref)"))
  ; Enable interactions on item upon entering collision zone
  (bind _ascharacter (cast `Character` OtherActor))
  (bind _isnpc (`self.IsPlayer` _ascharacter)
    (:`true`
      (`SceneComponent.SetVisibility` (`self.Widget`) true false)
      (`self.EnableInput` (`GameplayStatics.GetPlayerController` 0))
      ; If player is not NPC, enable ownership of the item for server side handling/destruction
      (set `self.Player` _ascharacter))
    (:`false`
      _))
  (if _isnpc
    (`self.SetOwner` _ascharacter)))

(event `self.SphereComponent.OnComponentEndOverlap`
  (params (OverlappedComponent :type "PrimitiveComponent Object Reference") (OtherActor :type "Actor Object Reference") (OtherComp :type "PrimitiveComponent Object Reference") (OtherBodyIndex :type Integer))
  ; Disables interaction on Item when leaving collision zone
  (bind _ascharacter (cast `Character` OtherActor))
  (`self.IsPlayer` _ascharacter
    (:`true`
      (`SceneComponent.SetVisibility` (`self.Widget`) false false)
      (`self.DisableInput` (`GameplayStatics.GetPlayerController` 0)))))

(fn `AddToInventory_WIP`
  (locals (FoundInventoryIndex_WIP :type Integer :default -1))
  (bind _id (`self.ID`))
  (bind _foundinventoryindex_wip (`local.FoundInventoryIndex_WIP`))
  (bind _returnvalue (>= _foundinventoryindex_wip 0))
  (bind _asbp_game_state_base (cast `/Game/Systems/BP_GameStateBase` (`GameplayStatics.GetGameState`))
    (:`then`
      (bind _inventory_wip (`/Game/Systems/BP_GameStateBase.Inventory_WIP` _asbp_game_state_base))
      (for (_array_element _array_index) _inventory_wip
        (if (== (`.PickupItemID_2_3E965EB4449FE3267E33A3BF34BC489A` (break `/Game/Systems/ST_InventorySlot_WIP` _array_element)) _id)
          (set `local.FoundInventoryIndex_WIP` _array_index)
          (break)))
      (if _returnvalue
        (bind _returnvalue_2 (`KismetMathLibrary.SelectInt` (+ (`.Amount_5_78C76B7942B6B4EB598E6AB1AFB82BD2` (break `/Game/Systems/ST_InventorySlot_WIP` (`|GetArrayItem` _inventory_wip _foundinventoryindex_wip))) 1) 1 _returnvalue))
        (bind _st_inventoryslot_wip (make `/Game/Systems/ST_InventorySlot_WIP` _id _returnvalue_2))
        (`KismetArrayLibrary.Array_Set` _inventory_wip _foundinventoryindex_wip _st_inventoryslot_wip _returnvalue)
        (else
          (`KismetArrayLibrary.Array_Add` _inventory_wip _st_inventoryslot_wip)))
      (`/Game/Utils/BPFL_Logging.Info` self (`|FormatText` "{Action} | ItemID: {ID} | Amount {Amount}" (`KismetMathLibrary.SelectText` "Updated item in inventory." "Added item to inventory." _returnvalue) _id _returnvalue_2) "AddToInventory_WIP"))
    (:`CastFailed`
      (`/Game/Utils/BPFL_Logging.Warn` self "Failed to get GameState." "AddToInventory_WIP"))))

(fn `Initialize`
  (bind _id (`self.ID`))
  (bind _pickupmeshcomponent (`self.PickupMeshComponent`))
  (bind _spherecomponent (`self.SphereComponent`))
  (bind _returnvalue (`|GetDataTableRow` (`self.ItemDataTable`) _id)
    (:`then`
      (bind _output_get (set `self.ReferenceItem` (`.Definition_11_8158F8FE468F141EE5B889BF9F2ED7B2` (break `/Game/Systems/ItemSystem/Data/ST_ItemData` _returnvalue))))
      (`StaticMeshComponent.SetStaticMesh` _pickupmeshcomponent (`/Game/Systems/ItemSystem/Data/DA_ItemDefinition.WorldMesh` _output_get))
      (`PrimitiveComponent.SetCollisionEnabled` _pickupmeshcomponent "NoCollision")
      (`PrimitiveComponent.SetCollisionEnabled` _spherecomponent "QueryOnly")
      (`SceneComponent.SetVisibility` _spherecomponent false false))
    (:`RowNotFound`
      (`/Game/Utils/BPFL_Logging.Warn` self (`|FormatText` "Unable to find row for item with ID: {id}" _id) "Initialize"))))

(fn `OnRep_ID`
  (bind _returnvalue (`|GetDataTableRow` "/Game/Systems/ItemSystem/DT_ItemData.DT_ItemData" (`self.ID`))
    (:`then`
      (set `self.Item` (select `bool` (!= (`.ID_15_5B3A2782400A599D58761E8D9F5308D4` (break `/Game/Systems/ItemSystem/Data/ST_ItemData` (`self.DroppedItem`))) "None") :`false` _returnvalue :`true` (`self.DroppedItem`)))
      (`self.Update`))))

(fn `UserConstructionScript`
  (`self.Initialize`))