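; Base world item actor for the item system, showing the static mesh that matches its item ID.
; On BeginPlay, Initialize sets the mesh from a data table row, then calls the ID's RepNotify directly.
; OnRep_ID looks up DT_ItemData, preferring DroppedItem data when that is set to distinguish drops from spawns.
; Update then blocking-loads the item definition's mesh asset and applies it; missing rows log warnings.
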(event `Update`
  ; Update item mesh when ID changed
  (bind _returnvalue (`KismetSystemLibrary.LoadAsset_Blocking` (`|ConvertAsset` (`.Definition_11_8158F8FE468F141EE5B889BF9F2ED7B2` (break `/Game/Systems/ItemSystem/Data/ST_ItemData` (`self.Item`))))))
  (bind _asstatic_mesh (cast `StaticMesh` _returnvalue))
  (`StaticMeshComponent.SetStaticMesh` (`self.ItemMesh`) _asstatic_mesh))

(event `self.ReceiveBeginPlay`
  ; Calls the item replication function when pickup starts
  (`self.Initialize`)
  (`self.OnRep_ID`))

(fn `Initialize`
  (bind _id (`self.ID`))
  ; Load item mesh
  (bind _returnvalue (`|GetDataTableRow` (`self.DataTable`) _id)
    (:`then`
      (bind _output_get (set `self.ReferenceItem` (`.Definition_11_8158F8FE468F141EE5B889BF9F2ED7B2` (break `/Game/Systems/ItemSystem/Data/ST_ItemData` _returnvalue))))
      (`StaticMeshComponent.SetStaticMesh` (`self.ItemMesh`) (`/Game/Systems/ItemSystem/Data/DA_ItemDefinition.WorldMesh` _output_get)))
    (:`RowNotFound`
      (`/Game/Utils/BPFL_Logging.Warn` self (`|FormatText` "Unable to find row for item with ID: {id}" _id) "Initialize"))))

(fn `OnRep_ID`
  (bind _id (`self.ID`))
  ; On item ID changed, check if Item was dropped or spawned
  (bind _returnvalue (`|GetDataTableRow` "/Game/Systems/ItemSystem/DT_ItemData.DT_ItemData" _id)
    (:`then`
      (set `self.Item` (select `bool` (!= (`.ID_15_5B3A2782400A599D58761E8D9F5308D4` (break `/Game/Systems/ItemSystem/Data/ST_ItemData` (`self.DroppedItem`))) "None") :`false` _returnvalue :`true` (`self.DroppedItem`)))
      (`self.Update`))
    (:`RowNotFound`
      (`/Game/Utils/BPFL_Logging.Warn` self (`|FormatText` "Unable to find row for item with ID: {id}" _id) "Initialize"))))

(fn `UserConstructionScript`)