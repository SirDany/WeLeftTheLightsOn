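; Ship-system job terminal actor that the player can open when nearby to take, complete or abandon jobs.
; An overlap sphere toggles the prompt, input and the controller's in-range flag.
; It relays GameState job and ship updates through its own calls and routes Terminal UI actions to job functions.
; Job generation appends three random data-table rows to a list, running shortly after BeginPlay and after each completion or abandonment.
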(event `self.ReceiveBeginPlay`
  ; Bind terminal update on state changes
  (bind _asbp_game_state_base (cast `/Game/Systems/BP_GameStateBase` (`GameplayStatics.GetGameState`))
    (:`then`
      (add `/Game/Systems/BP_GameStateBase.OnJobStateUpdated` _asbp_game_state_base (delegate `Jobs Updated`))
      (add `/Game/Systems/BP_GameStateBase.OnShipStateUpdated` _asbp_game_state_base (delegate `Ship Updated`))
      ; Set interact prompt
      (bind _aswbp_pickup (cast `/Game/Systems/UI/Widgets/WBP_Pickup` (`WidgetComponent.GetWidget` (`self.InteractPrompt`))))
      (`/Game/Systems/UI/Widgets/WBP_Pickup.UpdateActionPrompt` _aswbp_pickup "Open Terminal")
      (`KismetSystemLibrary.Delay` 0.2)
      (`self.GenerateRandomJobs`))
    (:`CastFailed`
      (`/Game/Utils/BPFL_Logging.Error` null "Unable to bind job terminal refresh to GameState."))))

(event `Jobs Updated`
  (params (JobState :type "/Game/Systems/JobSystem/ST_JobState Structure"))
  ; Bind terminal update on state changes
  (`self.OnJobsUpdated` JobState))

(event `Ship Updated`
  (params (ShipState :type "/Game/Systems/ShipSystem/ST_ShipState Structure"))
  ; Bind terminal update on state changes
  (`self.OnShipUpdated` ShipState))

(event `OnUIAction`
  (params (UIAction :type "/Game/Systems/UI/S_UIAction Structure"))
  (bind (_uiaction _uiwindowid _contextdata) (break `/Game/Systems/UI/S_UIAction` UIAction))
  (switch `/Game/Systems/UI/E_UIType` _uiwindowid
    (:`NewEnumerator1`
      (switch `/Game/Systems/UI/Data/E_UIActionType` _uiaction
        (:`NewEnumerator3`
          (`/Game/Systems/JobSystem/BPFL_JobService.SetActiveJob` _contextdata))
        (:`NewEnumerator4`
          (`/Game/Systems/JobSystem/BPFL_JobService.CompleteActiveJob`)
          (`self.GenerateRandomJobs` :!label _label))
        (:`NewEnumerator5`
          (`/Game/Systems/JobSystem/BPFL_JobService.AbandonActiveJob`)
          (goto _label))))))

(event `self.SphereComponent.OnComponentBeginOverlap`
  (params (OverlappedComponent :type "PrimitiveComponent Object Reference") (OtherActor :type "Actor Object Reference") (OtherComp :type "PrimitiveComponent Object Reference") (OtherBodyIndex :type Integer) (bFromSweep :type Boolean) (SweepResult :type "HitResult Structure (by ref)"))
  (bind _returnvalue (`GameplayStatics.GetPlayerController` 0))
  ; Enable interactions on item upon entering collision zone
  (bind _ascharacter (cast `Character` OtherActor))
  (bind _isplayer (`/Game/Systems/InteractUtils.IsPlayer` _ascharacter))
  (if _isplayer
    (`SceneComponent.SetVisibility` (`self.InteractPrompt`) true false)
    (`self.EnableInput` _returnvalue)
    (bind _asbp_first_person_player_controller (cast `/Game/FirstPerson/Blueprints/BP_FirstPersonPlayerController` _returnvalue))
    (set `/Game/FirstPerson/Blueprints/BP_FirstPersonPlayerController.IsInTerminalRange` true _asbp_first_person_player_controller)))

(event `self.SphereComponent.OnComponentEndOverlap`
  (params (OverlappedComponent :type "PrimitiveComponent Object Reference") (OtherActor :type "Actor Object Reference") (OtherComp :type "PrimitiveComponent Object Reference") (OtherBodyIndex :type Integer))
  (bind _returnvalue (`GameplayStatics.GetPlayerController` 0))
  ; Disables interaction on Item when leaving collision zone
  (bind _ascharacter (cast `Character` OtherActor))
  (bind _isplayer (`/Game/Systems/InteractUtils.IsPlayer` _ascharacter))
  (if _isplayer
    (`SceneComponent.SetVisibility` (`self.InteractPrompt`) false false)
    (`self.DisableInput` _returnvalue)
    (bind _asbp_first_person_player_controller (cast `/Game/FirstPerson/Blueprints/BP_FirstPersonPlayerController` _returnvalue))
    (set `/Game/FirstPerson/Blueprints/BP_FirstPersonPlayerController.IsInTerminalRange` false _asbp_first_person_player_controller)))

(fn `GenerateRandomJobs`
  (locals (JobDataToGenerate :type "Array of /Game/Systems/JobSystem/Data/ST_JobData Structure"))
  (bind _jobdata (`self.JobData`))
  (bind _outrownames (`DataTableFunctionLibrary.GetDataTableRowNames` _jobdata))
  (for _ (range 1 (+ 3 1))
    (bind _returnvalue (`|GetDataTableRow` _jobdata (`KismetArrayLibrary.Array_Random` _outrownames))
      (:`then`
        (`KismetArrayLibrary.Array_Add` (`local.JobDataToGenerate`) _returnvalue))))
  (`/Game/Systems/JobSystem/BPFL_JobService.GenerateAvailableJobs` 1.0 true (`local.JobDataToGenerate`)))

(fn `GetInteractionKey`
  (params (Key :type "InputAction Object Reference"))
  (returns (Success :type Boolean))
  (return false))

(fn `GetInteractionPrompt`
  (params (Prompt :type Text))
  (returns (Success :type Boolean))
  (return false))

(fn `TriggerUpdates`)

(fn `UserConstructionScript`)