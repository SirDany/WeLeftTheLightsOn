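; Game state Blueprint that stores the current job and ship states, exposing getter and update functions for each.
; On BeginPlay it binds to the item pickup event and passes each picked-up item ID and amount to UpdateJobProgress, which is defined outside these graphs.
; A successful progress update writes an info log marked as temporary.
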(event `self.ReceiveBeginPlay`
  (add `self.OnItemPickup` (delegate `Event OnItemPickup`)))

(event `Event OnItemPickup` :!signature `self.OnItemPickup`
  (params (ItemID :type Name) (Amount :type Integer))
  (bind _success (`/Game/Systems/JobSystem/BPFL_JobService.UpdateJobProgress` ItemID Amount))
  ; Remove this later
  (if _success
    (`/Game/Utils/BPFL_Logging.Info` self "Updated Job Progress!" "OnItemPickup")))

(fn `GetJobState`
  (returns (JobState :type "/Game/Systems/JobSystem/ST_JobState Structure"))
  (return (`self.JobState`)))

(fn `GetShipState`
  (returns (ShipState :type "/Game/Systems/ShipSystem/ST_ShipState Structure"))
  (return (`self.ShipState`)))

(fn `UpdateJobState`
  (params (JobState :type "/Game/Systems/JobSystem/ST_JobState Structure"))
  (set `self.JobState` JobState))

(fn `UpdateShipState`
  (params (ShipState :type "/Game/Systems/ShipSystem/ST_ShipState Structure"))
  (set `self.ShipState` ShipState))

(fn `UserConstructionScript`)