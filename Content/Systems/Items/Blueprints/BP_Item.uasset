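; BP_Item is a data-driven item actor that builds itself from a replicated ID on construction and on replication.
; The ID looks up a DT_ItemData row and blocking-loads its DA_ItemDefinition.
; Component classes from the definition are added when their supported tags match the item's tags, and the first able component renders the mesh.
; Input checks, available interactions and interactions delegate to the added components and combine their results.
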(fn `CanHandleInput`
  (params (Input :type "InputAction Object Reference"))
  (returns (CanHandle :type Boolean))
  (bind _valuepin (`|SetForEach` (`self.AddedComponents`))
    (:`then`
      (bind _asac_interactable_item_component (cast `/Game/Systems/Items/Components/AC_InteractableItemComponent` _valuepin))
      (bind _canhandle (`/Game/Systems/Items/Components/AC_InteractableItemComponent.CanHandleInput` _asac_interactable_item_component Input))
      (if _canhandle
        (return true)))
    (:`CompletedPin`
      (return false))))

(fn `GetAvailableInteractions`
  (returns (Interactions :type "Map of InputAction Object Reference to Text"))
  (locals (CummInteractions :type "Map of InputAction Object Reference to Text"))
  (bind _valuepin (`|SetForEach` (`self.AddedComponents`))
    (:`then`
      (bind _interactions (message `/Game/Systems/UI/BPI_Interactable.GetAvailableInteractions` _valuepin))
      (bind (_keypin _valuepin_2) (`|MapForEach` _interactions)
        (:`then`
          (`BlueprintMapLibrary.Map_Add` (`local.CummInteractions`) _keypin _valuepin_2))))
    (:`CompletedPin`
      (return (`local.CummInteractions`)))))

(fn `Initialize`
  (bind _id (`self.ID`))
  (bind _returnvalue (`|GetDataTableRow` "/Game/Systems/Items/Data/DT_ItemData.DT_ItemData" _id)
    (:`then`
      (bind _returnvalue_2 (`KismetSystemLibrary.LoadAsset_Blocking` (`|ConvertAsset` (`.Definition_11_8158F8FE468F141EE5B889BF9F2ED7B2` (break `/Game/Systems/Items/Data/ST_ItemData` _returnvalue)))))
      (bind _asda_item_definition (cast `/Game/Systems/Items/Data/DA_ItemDefinition` _returnvalue_2)
        (:`then`
          (set `self.ItemDefinition` _asda_item_definition))
        (:`CastFailed`
          (`/Game/Utils/BPFL_Logging.Warn` self (`|FormatText` "Unable to find definition for item with ID: {id}" _id) "OnRep_ID"))))
    (:`RowNotFound`
      (`/Game/Utils/BPFL_Logging.Warn` self (`|FormatText` "Unable to find row for item with ID: {id}" _id) "OnRep_ID"))))

(fn `Interact`
  (params (Controller :type "Controller Object Reference") (Input :type "InputAction Object Reference"))
  (returns (RemoveInteractable :type Boolean) (PlaySound :type "SoundBase Object Reference"))
  (locals (RemoveFromInteractables :type Boolean) (SoundToPlay :type "SoundBase Object Reference"))
  (bind _valuepin (`|SetForEach` (`self.AddedComponents`))
    (:`then`
      (bind (_removeinteractable _playsound) (message `/Game/Systems/UI/BPI_Interactable.Interact` _valuepin Controller Input))
      (set `local.RemoveFromInteractables` (or _removeinteractable (`local.RemoveFromInteractables`)))
      (`/Engine/EditorBlueprintResources/StandardMacros.IsValid` _playsound
        (:`Is Valid`
          (set `local.SoundToPlay` _playsound))))
    (:`CompletedPin`
      (return (`local.RemoveFromInteractables`) (`local.SoundToPlay`)))))

(fn `LoadComponents`
  (bind _addedcomponents (`self.AddedComponents`))
  ; Clean up existing components
  (bind _valuepin (`|SetForEach` _addedcomponents)
    (:`then`
      (`ActorComponent.K2_DestroyComponent` _valuepin)
      (`BlueprintSetLibrary.Set_Clear` _addedcomponents))
    (:`CompletedPin`
      ; Add new components based on tags
      (bind _valuepin_2 (`|SetForEach` (`/Game/Systems/Items/Data/DA_ItemDefinition.Components` (`self.ItemDefinition`)))
        (:`then`
          (bind _asac_item_component (castclass `/Game/Systems/Items/Components/AC_ItemComponent` _valuepin_2)
            (:`then`
              (if (`BlueprintGameplayTagLibrary.HasAnyTags` (`/Game/Systems/Items/Data/DA_ItemDefinition.Tags` (`self.ItemDefinition`)) (defaults `Object` _asac_item_component) true)
                (bind _returnvalue (`|AddComponentByClass` _valuepin_2))
                (`BlueprintSetLibrary.Set_Add` (`self.AddedComponents`) _returnvalue)
                (else
                  (`/Game/Utils/BPFL_Logging.Warn` self (`|FormatText` "Could not add component of class {component}" (`KismetSystemLibrary.GetClassDisplayName` _valuepin_2)) "LoadComponents" :!label _label))))
            (:`CastFailed`
              (goto _label))))))))

(fn `OnRep_ID`
  (if (!= (`self.ID`) "None")
    (`self.Initialize`)
    (`self.LoadComponents`)
    (`self.RenderItem`)))

(fn `RenderItem`
  (for _array_element (`self.K2_GetComponentsByClass` "/Game/Systems/Items/Components/AC_ItemComponent.AC_ItemComponent_C")
    (bind _rendersitem (`/Game/Systems/Items/Components/AC_ItemComponent.CanRenderItem` _array_element))
    (if _rendersitem
      (`/Game/Systems/Items/Components/AC_ItemComponent.RenderItem` _array_element (`self.ItemMesh`))
      (break))))

(fn `UserConstructionScript`
  (`self.OnRep_ID`))