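; Base item actor that displays the world mesh for the item identified by its replicated ID.
; The ID's OnRep, also run on construction and BeginPlay, looks up the row in DT_ItemData, stores it as Item and calls Update, warning if missing.
; Update synchronously loads the item's definition asset and applies its mesh, setting the relative transform only when no parent actor owns the item.
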(event `Update`
  (params (Item :type "/Game/Systems/Items/Data/ST_ItemData Structure"))
  (bind _itemmesh (`self.ItemMesh`))
  ; Update item mesh when ID changed
  (bind _returnvalue (`KismetSystemLibrary.LoadAsset_Blocking` (`|ConvertAsset` (`.Definition_11_8158F8FE468F141EE5B889BF9F2ED7B2` (break `/Game/Systems/Items/Data/ST_ItemData` Item)))))
  (bind _asda_item_definition (cast `/Game/Systems/Items/Data/DA_ItemDefinition` _returnvalue)
    (:`then`
      (`StaticMeshComponent.SetStaticMesh` _itemmesh (`/Game/Systems/Items/Data/DA_ItemDefinition.WorldMesh` _asda_item_definition))
      ; If owned by a parent, parent sets transform
      (if (not (`KismetSystemLibrary.IsValid` (`self.GetParentActor`)))
        (`SceneComponent.K2_SetRelativeTransform` _itemmesh (`/Game/Systems/Items/Data/DA_ItemDefinition.WorldTransform` _asda_item_definition) false false)))
    (:`CastFailed`
      (`KismetSystemLibrary.PrintString` "Item mesh loading failed on update"))))

(event `self.ReceiveBeginPlay`
  ; Calls the item replication function when pickup starts
  (`self.OnRep_ID`))

(fn `OnRep_ID`
  (bind _id (`self.ID`))
  ; On item ID changed, check if Item was dropped or spawned
  (bind _returnvalue (`|GetDataTableRow` "/Game/Systems/Items/Data/DT_ItemData.DT_ItemData" _id)
    (:`then`
      (bind _output_get (set `self.Item` _returnvalue))
      (`self.Update` _output_get))
    (:`RowNotFound`
      (`/Game/Utils/BPFL_Logging.Warn` self (`|FormatText` "Unable to find row for item with ID: {id}" _id) "OnRep_ID"))))

(fn `UserConstructionScript`
  (`self.OnRep_ID`))