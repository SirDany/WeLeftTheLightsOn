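; Planet generator actor that drives staged procedural planet generation alongside the PCG volumes in the level.
; Initialize respawns one actor per Stages class at its own transform; Cleanup forwards to each of them.
; Generate runs every stage actor, then force-generates all PCG volumes.
; BeginPlay only calls Generate and prints each volume's GenOrder, since the Cleanup and Initialize chain is disconnected.
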(event Custom|Generate
  (for _array_element (Variables|Default|GetStageActors)
    (Default|Generate _array_element))
  (bind _outactors (Actor|GetAllActorsOfClass "/Script/PCG.PCGVolume"))
  (for _array_element_2 _outactors
    (PCG|Generate (Variables|/Script/PCG.PCGVolume|GetPCGComponent _array_element_2) true)))

(event Custom|Initialize
  (bind _stageactors (Variables|Default|GetStageActors))
  (for _array_element _stageactors
    (Utilities|IsValid _array_element
      (:Is%20Valid
        (Actor|DestroyActor _array_element))))
  (Utilities|Array|Clear _stageactors)
  (for _array_element_2 (Variables|Default|GetStages)
    (bind _returnvalue (Game|SpawnActorfromClass _array_element_2 (Transformation|GetActorTransform) "Undefined" "MultiplyWithRoot" 0 0))
    (Utilities|Array|Add (Variables|Default|GetStageActors) _returnvalue)))

(event Custom|Cleanup
  (for _array_element (Variables|Default|GetStageActors)
    (Default|Cleanup _array_element)))

(event EventBeginPlay
  (CallFunction|Generate)
  (bind _outactors (Actor|GetAllActorsOfClass "/Script/PCG.PCGVolume"))
  (for _array_element _outactors
    (bind _returnvalue (Class|PCGGraphParametersHelpers|GetInt32Parameter (Variables|/Script/PCG.PCGComponent|GetGraphInstance (Variables|/Script/PCG.PCGVolume|GetPCGComponent _array_element)) "GenOrder"))
    (Development|PrintString (Utilities|String|ToString(Integer) _returnvalue))))

(fn ConstructionScript)