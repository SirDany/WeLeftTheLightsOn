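; Ship terminal actor that players interact with to toggle a terminal UI for managing jobs and buying energy.
; On BeginPlay it binds to GameState job and ship updates, relays them through its own dispatchers, then generates random jobs after a short delay.
; UI actions route to job manager and shop components.
; Completing or abandoning a job refreshes the available list from the job generator component.
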(event `self.ReceiveBeginPlay`
  (`parent.ReceiveBeginPlay`)
  ; Bind terminal update on state changes
  (bind _asbp_game_state_base (cast `/Game/Systems/BP_GameStateBase` (`GameplayStatics.GetGameState`))
    (:`then`
      (add `/Game/Systems/BP_GameStateBase.OnJobStateUpdated` _asbp_game_state_base (delegate `Jobs Updated`))
      (add `/Game/Systems/BP_GameStateBase.OnShipStateUpdated` _asbp_game_state_base (delegate `Ship Updated`))
      (`KismetSystemLibrary.Delay` 0.2)
      (`self.GenerateRandomJobs`))
    (:`CastFailed`
      (`/Game/Utils/BPFL_Logging.Error` self "Unable to bind job terminal refresh to GameState." "Begin Play"))))

(event `Jobs Updated`
  (params (JobState :type "/Game/Systems/Jobs/ST_JobState Structure"))
  ; Bind terminal update on state changes
  (`self.OnJobsUpdated` JobState))

(event `Ship Updated`
  (params (ShipState :type "/Game/Systems/Ship/ST_ShipState Structure"))
  ; Bind terminal update on state changes
  (`self.OnShipUpdated` ShipState))

(event `OnUIAction`
  (params (UIAction :type "/Game/Systems/UI/S_UIAction Structure"))
  (bind (_uiaction _uiwindowid _contextdata) (break `/Game/Systems/UI/S_UIAction` UIAction))
  (bind _ac_jobmanager (`self.AC_JobManager`))
  (switch `/Game/Systems/UI/E_UIType` _uiwindowid
    (:`NewEnumerator1`
      (switch `/Game/Systems/UI/Data/E_UIActionType` _uiaction
        (:`NewEnumerator3`
          (`/Game/Systems/Jobs/AC_JobManager.SetActiveJob` _ac_jobmanager _contextdata))
        (:`NewEnumerator4`
          (`/Game/Systems/Jobs/AC_JobManager.CompleteActiveJob` _ac_jobmanager)
          (`self.GenerateRandomJobs` :!label _label))
        (:`NewEnumerator5`
          (`/Game/Systems/Jobs/AC_JobManager.AbandonActiveJob` _ac_jobmanager)
          (goto _label))
        (:`NewEnumerator7`
          (`/Game/Systems/Ship/Terminal/AC_ShopComponent.BuyEnergy` (`self.AC_ShopComponent`) 100))))))

(fn `GenerateRandomJobs`
  (locals (JobDataToGenerate :type "Array of /Game/Systems/Jobs/Data/ST_JobData Structure"))
  (bind _jobs (`/Game/Systems/Jobs/AC_JobGenerator.GenerateJobs` (`self.AC_JobGenerator`) 3))
  (`/Game/Systems/Jobs/AC_JobManager.SetAvailableJobs` (`self.AC_JobManager`) _jobs))

(fn `Interact`
  (params (Controller :type "Controller Object Reference") (Input :type "InputAction Object Reference"))
  (returns (RemoveInteractable :type Boolean) (PlaySound :type "SoundBase Object Reference"))
  (bind _canhandle (`self.CanHandleInput` Input))
  (if _canhandle
    (bind _asbp_first_person_player_controller (cast `/Game/FirstPerson/Blueprints/BP_FirstPersonPlayerController` Controller))
    (`/Game/Systems/UI/AC_UIManager.ToggleUIWindow` (`/Game/FirstPerson/Blueprints/BP_FirstPersonPlayerController.UIManager` _asbp_first_person_player_controller) "NewEnumerator1" "Menu")
    (return false null)))

(fn `UserConstructionScript`)