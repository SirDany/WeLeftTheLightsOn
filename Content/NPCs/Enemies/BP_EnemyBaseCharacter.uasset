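; BP_EnemyBaseCharacter is a base enemy character Blueprint that tracks progress along a patrol route.
; It holds an array of patrol points and an index, and returns the point at that index as the current patrol target.
; The OnPatrolPointReached event advances the index, wrapping to zero after the last point so the route loops.
; The file contains no movement logic of its own.
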(event `OnPatrolPointReached`
  (`self.IncrementPatrolIndex`))

(fn `GetCurrentPatrolTarget`
  (returns (PatrolPoint :type "/Game/NPCs/Enemies/BP_PatrolPoint Object Reference"))
  (return (`|GetArrayItem` (`self.PatrolPoints`) (`self.PatrolIndex`))))

(fn `IncrementPatrolIndex`
  (bind _patrolindex (`self.PatrolIndex`))
  (`/Engine/EditorBlueprintResources/StandardMacros.IncrementInt` _patrolindex
    (:`  `
      (if (>= _patrolindex (`KismetArrayLibrary.Array_Length` (`self.PatrolPoints`)))
        (set `self.PatrolIndex` 0)))))

(fn `UserConstructionScript`)