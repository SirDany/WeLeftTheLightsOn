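; Player state Blueprint that holds the player's stats and announces when they change.
; On BeginPlay it builds the Stats array from a data table, starting each stat at its base max with base drain and recovery rates.
; UpdatePlayerStats merges incoming stats by type through a map, rebuilds the array, and fires OnPlayerStatsUpdated inside the update loop with the changed types.
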(event `self.ReceiveBeginPlay`
  (`self.InitializePlayerStats`))

(fn `InitializePlayerStats`
  (bind _output (`|ConvertAsset` (`self.PlayerStatsDataTable`)))
  (bind _outrownames (`DataTableFunctionLibrary.GetDataTableRowNames` _output))
  (for _array_element _outrownames
    (bind _returnvalue (`|GetDataTableRow` _output _array_element)
      (:`then`
        (bind (_basemax _basedrainrate _baserecoveryrate _playerstattype) (break `/Game/Players/StatSystem/BaseStats/ST_PlayerStatsRow` _returnvalue))
        (`KismetArrayLibrary.Array_Add` (`self.Stats`) (make `/Game/Players/StatSystem/ST_PlayerStat` _basemax _basemax _basedrainrate _baserecoveryrate _playerstattype))))))

(fn `UpdatePlayerStats`
  (params (NewPlayerStats :type "Array of /Game/Players/StatSystem/ST_PlayerStat Structure"))
  (locals (PlayerStatMap :type "Map of /Game/Players/StatSystem/BaseStats/EN_PlayerStatType Enum to /Game/Players/StatSystem/ST_PlayerStat Structure") (UpdatedStatTypes :type "Array of /Game/Players/StatSystem/BaseStats/EN_PlayerStatType Enum"))
  (bind _playerstatmap (`local.PlayerStatMap`))
  (bind _updatedstattypes (`local.UpdatedStatTypes`))
  ; Create map of current stats for simple lookup
  (for _array_element (`self.Stats`)
    (`BlueprintMapLibrary.Map_Add` _playerstatmap (`.Type_12_9D0B473A4B87CB9531C890AB77D992B4` (break `/Game/Players/StatSystem/ST_PlayerStat` _array_element)) _array_element))
  ; Update or add stats
  (for _array_element_2 NewPlayerStats
    (bind (_current _max _drainrate _recoveryrate _type) (break `/Game/Players/StatSystem/ST_PlayerStat` _array_element_2))
    (`BlueprintMapLibrary.Map_Add` _playerstatmap _type _array_element_2)
    (`KismetArrayLibrary.Array_Add` _updatedstattypes _type)
    (bind _values (`BlueprintMapLibrary.Map_Values` _playerstatmap))
    (bind _output_get (set `self.Stats` _values))
    (`self.OnPlayerStatsUpdated` _output_get _updatedstattypes) ; Ignore the pass by reference note, arrays will still be passed even as non reference.
  ))

(fn `UserConstructionScript`)