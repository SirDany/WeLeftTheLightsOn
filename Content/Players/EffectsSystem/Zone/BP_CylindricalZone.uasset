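; BP_CylindricalZone is a cylindrical area that periodically applies stacks of a configurable effect to players inside it.
; Overlap events track first-person characters in PlayersInZone, starting a looping timer on entry and clearing it when the zone empties.
; Each timer tick applies the effect through each character's BP_PlayerState and warns on failure.
; The construction script gives the cylinder a translucent dynamic material tinted with the zone's color.
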(event `ApplyEffectEvent`
  (for _array_element (`self.PlayersInZone`)
    (bind _asbp_player_state (cast `/Game/Players/BP_PlayerState` (`Pawn.PlayerState` _array_element)))
    (bind _success (`/Game/Players/EffectsSystem/BPFL_EffectService.ApplyEffect` _asbp_player_state (`self.EffectType`) (`self.StacksPerInterval`)))
    (if (not _success)
      (`/Game/Utils/BPFL_Logging.Warn` self "Failed to apply effect." "ApplyEffect Timer"))))

(event `self.ReceiveActorBeginOverlap`
  (params (OtherActor :type "Actor Object Reference"))
  (bind _asbp_first_person_character (cast `/Game/FirstPerson/Blueprints/BP_FirstPersonCharacter` OtherActor))
  (`KismetArrayLibrary.Array_Add` (`self.PlayersInZone`) _asbp_first_person_character)
  (if (not (`KismetSystemLibrary.K2_IsTimerActiveHandle` (`self.Timer`)))
    (bind _returnvalue (`KismetSystemLibrary.K2_SetTimerDelegate` (delegate `ApplyEffectEvent`) (`self.IntervalSeconds`) true))
    (set `self.Timer` _returnvalue)))

(event `self.ReceiveActorEndOverlap`
  (params (OtherActor :type "Actor Object Reference"))
  (bind _timer (`self.Timer`))
  (bind _asbp_first_person_character (cast `/Game/FirstPerson/Blueprints/BP_FirstPersonCharacter` OtherActor))
  (`KismetArrayLibrary.Array_RemoveItem` (`self.PlayersInZone`) _asbp_first_person_character)
  (if (and (`KismetArrayLibrary.Array_IsEmpty` (`self.PlayersInZone`)) (`KismetSystemLibrary.K2_IsTimerActiveHandle` _timer))
    (`KismetSystemLibrary.K2_ClearAndInvalidateTimerHandle` _timer)))

(fn `UserConstructionScript`
  (bind _returnvalue (`KismetMaterialLibrary.CreateDynamicMaterialInstance` "/Game/Players/EffectsSystem/Zone/M_ZoneTransparent.M_ZoneTransparent"))
  (`MaterialInstanceDynamic.SetVectorParameterValue` _returnvalue "ZoneColor" (`self.Color`))
  (`MaterialInstanceDynamic.SetScalarParameterValue` _returnvalue "Opacity" 0.3)
  (`PrimitiveComponent.SetMaterial` (`self.Cylinder`) 0 _returnvalue))